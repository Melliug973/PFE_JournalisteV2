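; Waterfall spline actor that moves Niagara emitters along a spline in a continuous flow, with a splash sound.
; The construction script spawns NumberOfEmitters Niagara components evenly spaced along the spline.
; At BeginPlay a timeline starts from a random time at PlayRate, offsetting each emitter's wrapped spline distance on every update.
; The splash sound fires at the actor's location for every emitter on every update.
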(event `self.ReceiveBeginPlay`
  (`TimelineComponent.SetPlayRate` (`self.ParticleAnim`) (`self.PlayRate`))
  (`|ExecutionSequence`
    (:`then_0`
      (bind (_direction _anim) (`Timeline|ParticleAnim` :`NewTime` (`KismetMathLibrary.RandomFloat`) :!via `SetNewTime` :!label _label)
        (:`Update`
          (for (_array_element _array_index) (`self.Particles`)
            (`SceneComponent.K2_SetRelativeLocation` _array_element (`SplineComponent.GetLocationAtDistanceAlongSpline` (`self.Spline`) (* (mod (+ (* _array_index (/ 1.0 (`KismetMathLibrary.Conv_IntToDouble` (`self.NumberOfEmitters`)))) _anim) 1.0) (`SplineComponent.GetSplineLength` (`self.Spline`))) "Local") false false)
            (`GameplayStatics.PlaySoundAtLocation` "/Game/01_WorkShop/06_Sounds/Water/S_Water_Splash.S_Water_Splash" (`self.K2_GetActorLocation`) (struct) 1.0 1.0 0.0 null null null)))))
    (:`then_1`
      (goto _label))))

(fn `UserConstructionScript`
  (bind _numberofemitters (`self.NumberOfEmitters`))
  (for _index (range _numberofemitters)
    (bind _returnvalue (`AddComponent|NODE_AddNiagaraComponent-1` :`RelativeTransform` (`KismetMathLibrary.Conv_VectorToTransform` (`SplineComponent.GetLocationAtDistanceAlongSpline` (`self.Spline`) (* _index (/ (`SplineComponent.GetSplineLength` (`self.Spline`)) (`KismetMathLibrary.Conv_IntToDouble` _numberofemitters))) "Local"))))
    (`NiagaraComponent.SetAsset` _returnvalue (`self.NiagaraSystem`) true)
    (`KismetArrayLibrary.Array_Add` (`self.Particles`) _returnvalue)))