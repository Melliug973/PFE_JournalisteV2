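; BP_Cube_Head is a head Blueprint in the NPC photo test folder that keeps its Sphere component turned toward the player camera.
; Each Tick sets the Sphere's world rotation with a look-at from its location to the camera manager's location.
; BeginPlay hides the Sphere, WidgetFace and Plane components without propagating to children.
; A WasRecentlyRendered debug print is left unconnected and never runs.
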(event `self.ReceiveTick`
  (params (DeltaSeconds :type "Float (single-precision)"))
  (bind _sphere (`self.Sphere`))
  (`SceneComponent.K2_SetWorldRotation` _sphere (`KismetMathLibrary.FindLookAtRotation` (`SceneComponent.K2_GetComponentLocation` _sphere) (`SceneComponent.K2_GetComponentLocation` (`PlayerCameraManager.TransformComponent` (`GameplayStatics.GetPlayerCameraManager` 0)))) false false))

(event `self.ReceiveBeginPlay`
  (`SceneComponent.SetVisibility` (`self.Sphere`) false false)
  (`SceneComponent.SetVisibility` (`self.WidgetFace`) false false)
  (`SceneComponent.SetVisibility` (`self.Plane`) false false))

(fn `UserConstructionScript`)