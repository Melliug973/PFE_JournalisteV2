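; Test NPC Blueprint that smoothly turns to face the third-person player character when within a short range.
; On BeginPlay it caches the player reference and starts a distance check that sets a rotate flag.
; The check and the facing event call each other and repeat through very short Delays instead of Tick.
; Facing interpolates toward the look-at rotation and applies only the yaw.
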(event `self.ReceiveBeginPlay`
  (bind _asbp_third_person_character (cast `/Game/ThirdPerson/Blueprints/BP_ThirdPersonCharacter` (`GameplayStatics.GetPlayerCharacter` 0)))
  (set `self.As BP Third Person Character` _asbp_third_person_character)
  (`self.Should Rotate`))

(event `Face Player`
  (bind (_returnvalue_roll _returnvalue_pitch _returnvalue_yaw) (`KismetMathLibrary.BreakRotator` (`KismetMathLibrary.RInterpTo` (`self.K2_GetActorRotation`) (`KismetMathLibrary.FindLookAtRotation` (`self.K2_GetActorLocation`) (`self.K2_GetActorLocation` (`self.As BP Third Person Character`))) (`GameplayStatics.GetWorldDeltaSeconds`) 5.0)))
  ;[1 1 1] Face Player
  (if (`self.Should Rotate?`)
    (`self.K2_SetActorRotation` (`KismetMathLibrary.MakeRotator` 0.0 0.0 _returnvalue_yaw))
    (`KismetSystemLibrary.Delay` 0.001)
    (`self.Face Player`)
    (else
      (`self.Should Rotate`))))

(event `Should Rotate`
  ;[1 1 1] Check should rotate
  (if (<= (`self.GetDistanceTo` (`self.As BP Third Person Character`)) 500.0)
    (set `self.Should Rotate?` true)
    (`self.Face Player`)
    (else
      (set `self.Should Rotate?` false)))
  (`KismetSystemLibrary.Delay` 0.001)
  (`self.Should Rotate`))

(fn `UserConstructionScript`)