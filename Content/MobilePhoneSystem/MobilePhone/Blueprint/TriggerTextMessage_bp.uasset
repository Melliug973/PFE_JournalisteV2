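; Trigger volume actor for the mobile phone system that shows a new text message notification when the player enters.
; While the character is inside with at least two RJText entries, Tick fires once, playing a ringtone, showing the widget and enabling MailButtonJournalActiv.
; Contact data comes from a newly created, not loaded, Mobilephone_save object.
; Limitpreviewtextamount builds a truncated preview from MessageDatatable but returns the full IntroMessage.
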(event `self.Box.OnComponentBeginOverlap`
  (params (OverlappedComponent :type "PrimitiveComponent Object Reference") (OtherActor :type "Actor Object Reference") (OtherComp :type "PrimitiveComponent Object Reference") (OtherBodyIndex :type Integer) (bFromSweep :type Boolean) (SweepResult :type "HitResult Structure (by ref)"))
  ;[1 1 1] Trigger Text Notifcation
  (bind _asbp_third_person_character (cast `/Game/ThirdPerson/Blueprints/BP_ThirdPersonCharacter` OtherActor))
  (set `self.IsInside ` true))

(event `self.ReceiveTick`
  (params (DeltaSeconds :type "Float (single-precision)"))
  (bind _contacts (`/Game/MobilePhoneSystem/MobilePhone/Blueprint/Mobilephone_save.contacts` (`self.NewVar`)))
  (bind (_output_name _output_contactimage _output_firstdialogue) (break `/Game/MobilePhoneSystem/MobilePhone/Blueprint/Contacts_Struct` (`|GetArrayItem` _contacts (`self.messagelist`))))
  ;[1 1 1] Trigger Text Notifcation
  (if (`self.IsInside `)
    (if (>= (`KismetArrayLibrary.Array_Length` (`/Game/ThirdPerson/Blueprints/BP_ThirdPersonCharacter.RJText` (stale `self.Box.OnComponentBeginOverlap` _asbp_third_person_character))) 2)
      (if (`self.Condition`)
        (set `self.Condition` false)
        (bind _returnvalue (`GameplayStatics.CreateSaveGameObject` "/Game/MobilePhoneSystem/MobilePhone/Blueprint/Mobilephone_save.Mobilephone_save_C"))
        (bind _output_get (set `self.NewVar` _returnvalue))
        (`GameplayStatics.PlaySound2D` (`/Game/MobilePhoneSystem/MobilePhone/Blueprint/Mobilephone_save.Ringtones` _output_get) 1.0 1.0 0.0 null null)
        (bind _returnvalue_2 (`self.Limitpreviewtextamount` _output_firstdialogue (`self.Previewtextamount`)))
        (bind _returnvalue_3 (`|CreateWidget` "/Game/MobilePhoneSystem/MobilePhone/Apps/MessageNotifcation_WB.MessageNotifcation_WB_C" null _output_contactimage _output_name _returnvalue_2 (`self.Delaytime`)))
        (`UserWidget.AddToViewport` _returnvalue_3 0)
        (`KismetArrayLibrary.Array_Set` _contacts (`self.messagelist`) (make `/Game/MobilePhoneSystem/MobilePhone/Blueprint/Contacts_Struct` _output_name _output_contactimage _output_firstdialogue))
        (set `/Game/ThirdPerson/Blueprints/BP_ThirdPersonCharacter.MailButtonJournalActiv` true (stale `self.Box.OnComponentBeginOverlap` _asbp_third_person_character))))))

(event `self.Box.OnComponentEndOverlap`
  (params (OverlappedComponent :type "PrimitiveComponent Object Reference") (OtherActor :type "Actor Object Reference") (OtherComp :type "PrimitiveComponent Object Reference") (OtherBodyIndex :type Integer))
  ;[1 1 1] Trigger Text Notifcation
  (cast `/Game/ThirdPerson/Blueprints/BP_ThirdPersonCharacter` OtherActor)
  (set `self.IsInside ` false))

(fn `Limitpreviewtextamount`
  (params (RowName :type Name) (PreviewTextAmount :type Integer))
  (returns (ReturnValue :type Text))
  (bind _returnvalue (`|GetDataTableRow` "/Game/MobilePhoneSystem/MobilePhone/Blueprint/MessageDatatable.MessageDatatable" RowName)
    (:`then`
      (set `self.Blank text` "")
      (for (_array_element _array_index) (`KismetStringLibrary.GetCharacterArrayFromString` (`KismetTextLibrary.Conv_TextToString` (break `/Game/MobilePhoneSystem/MobilePhone/Blueprint/DialogueSystem_Struct` _returnvalue)))
        (if (not (> _array_index PreviewTextAmount))
          (set `self.Blank text` (`KismetStringLibrary.Concat_StrStr` (`self.Blank text`) _array_element))))
      (bind _output_get (set `self.First msg line` (`KismetStringLibrary.Concat_StrStr` (`self.Blank text`) "...."))))
    (:`RowNotFound`
      _))
  (return (break `/Game/MobilePhoneSystem/MobilePhone/Blueprint/DialogueSystem_Struct` _returnvalue)))

(fn `UserConstructionScript`)