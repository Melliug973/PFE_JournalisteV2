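; Trigger volume actor that starts an incoming phone call when the player walks into it.
; On the first box overlap by a BP_ThirdPersonCharacter, it reaches the phone UI through the character's MobilePhoneComponent.
; If that UI is valid, it tells the notification widget someone is calling, passing the configured caller audio and name.
; A DoOnce limits it to a single call.
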(event `self.Box.OnComponentBeginOverlap`
  (params (OverlappedComponent :type "PrimitiveComponent Object Reference") (OtherActor :type "Actor Object Reference") (OtherComp :type "PrimitiveComponent Object Reference") (OtherBodyIndex :type Integer) (bFromSweep :type Boolean) (SweepResult :type "HitResult Structure (by ref)"))
  ;[1 1 1] Trigger phone call
  (bind _asbp_third_person_character (cast `/Game/ThirdPerson/Blueprints/BP_ThirdPersonCharacter` OtherActor))
  (`/Engine/EditorBlueprintResources/StandardMacros.DoOnce` false
    (:`Completed`
      (bind _phoneui (`/Game/MobilePhoneSystem/MobilePhone/Components/MobilePhoneComponent.phoneui` (`/Game/ThirdPerson/Blueprints/BP_ThirdPersonCharacter.MobilePhoneComponent` _asbp_third_person_character)))
      (`/Engine/EditorBlueprintResources/StandardMacros.IsValid` _phoneui
        (:`Is Valid`
          (`/Game/MobilePhoneSystem/MobilePhone/Apps/PhoneNotfication_WB.Someone is caling` (`/Game/MobilePhoneSystem/MobilePhone/Apps/Phoneui_WB.PhoneNotfication_WB` _phoneui) (`self.Calleraudio`) (`self.Callername`)))))))

(fn `UserConstructionScript`)