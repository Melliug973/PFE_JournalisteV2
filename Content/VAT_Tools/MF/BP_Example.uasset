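; Example actor for vertex animation textures that shows a data asset's mesh as an instanced static mesh and switches between two animations.
; The construction script adds the instance, and pressing I flips the animation index and plays a timeline.
; Timeline updates write start frame, length, playrate, looping and time offset into per-instance custom data, alongside the track value.
; Construction-time setup and manual frame-calculation chains are left unconnected.
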(event `self.ReceiveTick`
  (params (DeltaSeconds :type "Float (single-precision)")))

(event `self.ReceiveBeginPlay`
  (`self.EnableInput` (`GameplayStatics.GetPlayerController` 0)))

(event `Key|I`
  (params (Key :type "Key Structure"))
  (bind _instancedstaticmesh (`self.InstancedStaticMesh`))
  (bind _instancedstaticmesh_2 (`self.InstancedStaticMesh`))
  (bind (_output_startframe _output_endframe) (break `AnimToTextureAnimInfo` (`|GetArrayItem` (`AnimToTextureDataAsset.Animations` (`self.DataAsset`)) (`self.Anim Index`))))
  (bind _returnvalue (`KismetMathLibrary.Conv_IntToDouble` _output_startframe))
  (:`Pressed`
    (`/Engine/EditorBlueprintResources/StandardMacros.FlipFlop`
      (:`A`
        (set `self.Anim Index` 0)
        (bind (_direction _newtrack_0) (`Timeline|Timeline` :!label _label)
          (:`Update`
            ;[1 1 1] Start Frame Anim
            (`InstancedStaticMeshComponent.SetCustomDataValue` _instancedstaticmesh 7 0 _newtrack_0 true)
            ;[1 1 1] Start Frame Anim
            (`InstancedStaticMeshComponent.SetCustomDataValue` _instancedstaticmesh_2 0 0 _returnvalue true)
            ;[1 1 1] End Frames Anim
            (`InstancedStaticMeshComponent.SetCustomDataValue` _instancedstaticmesh_2 0 1 (`KismetMathLibrary.Conv_IntToDouble` (- _output_endframe _output_startframe)) true)
            ;[1 1 1] Playrate
            (`InstancedStaticMeshComponent.SetCustomDataValue` _instancedstaticmesh_2 0 2 1.0 true)
            ;[1 1 1] Looping
            (`InstancedStaticMeshComponent.SetCustomDataValue` _instancedstaticmesh_2 0 3 1.0 true)
            ;[1 1 1] TimeStartOffset
            (`InstancedStaticMeshComponent.SetCustomDataValue` _instancedstaticmesh_2 0 4 0.0 true))
          (:`Finished`
            (`InstancedStaticMeshComponent.SetCustomDataValue` _instancedstaticmesh 8 0 _returnvalue true))))
      (:`B`
        (set `self.Anim Index` 1)
        (goto _label)))))

(fn `UserConstructionScript`
  (bind _instancedstaticmesh (`self.InstancedStaticMesh`))
  (`StaticMeshComponent.SetStaticMesh` _instancedstaticmesh (`AnimToTextureDataAsset.BP_GetStaticMesh` (`self.DataAsset`)))
  (`InstancedStaticMeshComponent.AddInstance` _instancedstaticmesh (`KismetMathLibrary.MakeTransform` (0.0 0.0 0.0)) false))