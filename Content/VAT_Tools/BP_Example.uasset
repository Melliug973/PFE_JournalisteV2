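; Example Blueprint for vertex animation texture (VAT) playback on an instanced static mesh.
; The construction script takes the mesh from a data asset, adds one instance and looks up the animation selected by AnimIndex.
; It writes start frame, frame span, play rate, looping and time offset into per-instance custom data, with no Blueprint tick logic.
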(fn `UserConstructionScript`
  (bind _instancedstaticmesh (`self.InstancedStaticMesh`))
  (bind _instancedstaticmesh_2 (`self.InstancedStaticMesh`))
  (bind (_output_startframe _output_endframe) (break `AnimToTextureAnimInfo` (`|GetArrayItem` (`AnimToTextureDataAsset.Animations` (`self.DataAsset`)) (`self.Anim Index`))))
  (`StaticMeshComponent.SetStaticMesh` _instancedstaticmesh_2 (`AnimToTextureDataAsset.BP_GetStaticMesh` (`self.DataAsset`)))
  (`InstancedStaticMeshComponent.AddInstance` _instancedstaticmesh_2 (`KismetMathLibrary.MakeTransform` (0.0 0.0 0.0)) false)
  ;[1 1 1] Start Frame Anim
  (`InstancedStaticMeshComponent.SetCustomDataValue` _instancedstaticmesh 0 0 (`KismetMathLibrary.Conv_IntToDouble` _output_startframe) false)
  ;[1 1 1] End Frames Anim
  (`InstancedStaticMeshComponent.SetCustomDataValue` _instancedstaticmesh 0 1 (`KismetMathLibrary.Conv_IntToDouble` (- _output_endframe _output_startframe)) false)
  ;[1 1 1] Playrate
  (`InstancedStaticMeshComponent.SetCustomDataValue` _instancedstaticmesh 0 2 1.0 false)
  ;[1 1 1] Looping
  (`InstancedStaticMeshComponent.SetCustomDataValue` _instancedstaticmesh 0 3 1.0 false)
  ;[1 1 1] TimeStartOffset
  (`InstancedStaticMeshComponent.SetCustomDataValue` _instancedstaticmesh 0 4 0.0 false))