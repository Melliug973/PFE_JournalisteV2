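; BP_Crowd is a VAT test Blueprint that builds a static crowd grid of instanced meshes at construction.
; It places Rows by Columns instances with seeded random X offset and yaw.
; Per-instance custom data receives hard-coded frame, playrate and loop values, with time offset written to index 5 despite its [4] label.
; Random data-asset animation lookup does not feed those values, and AnimToTexture batch-update nodes are left unwired.
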(fn `UserConstructionScript`
  (bind _instancedstaticmesh (`self.InstancedStaticMesh`))
  (bind _randomstream (`self.RandomStream`))
  (bind _maxangle (`self.MaxAngle`))
  (bind (_output_startframe _output_endframe) (break `AnimToTextureAnimInfo` (`|GetArrayItem` (`AnimToTextureDataAsset.Animations` (`self.DataAsset`)) (`self.Animindex`))))
  ;[1 1 1] Comment
  (`|ExecutionSequence`
    (:`then_0`
      (`StaticMeshComponent.SetStaticMesh` (`self.InstancedStaticMesh`) (`self.StaticMeshAsset`)))
    (:`then_1`
      (for _index (range (`self.Rows`))
        (for _index_2 (range (`self.Columns`))
          (`InstancedStaticMeshComponent.AddInstance` (`self.InstancedStaticMesh`) (`KismetMathLibrary.MakeTransform` (`KismetMathLibrary.MakeVector` (+ (* _index_2 (`self.ColDistance`)) (`KismetMathLibrary.RandomFloatInRangeFromStream` _randomstream 0.0 (`self.ShuffleAmount`))) (* _index (`self.RowDistance`))) (`KismetMathLibrary.MakeRotator` 0.0 0.0 (`KismetMathLibrary.RandomFloatInRangeFromStream` _randomstream (* _maxangle -1.0) _maxangle))) false))))
    (:`then_2`
      (for _index_3 (range (* (`self.Rows`) (`self.Columns`)))
        (bind _output_get (set `self.Struct Ref` (`MassTrafficInstancePlaybackLibrary.AnimStateFromDataAsset` (`self.DataAsset`) (`KismetMathLibrary.RandomIntegerInRangeFromStream` (`self.RandomStream`) 0 (- (`KismetArrayLibrary.Array_Length` (`AnimToTextureDataAsset.Animations` (`self.DataAsset`))) 1)))))
        (set `self.In String` (`KismetStringLibrary.Conv_IntToString` _output_endframe))
        ;;[1 1 1] Frame Offset [0]
        (`InstancedStaticMeshComponent.SetCustomDataValue` _instancedstaticmesh _index_3 0 90.0 false)
        ;;[1 1 1] NumFrames [1]
        (`InstancedStaticMeshComponent.SetCustomDataValue` _instancedstaticmesh _index_3 1 300.0 false)
        ;;[1 1 1] Playrate [2]
        (`InstancedStaticMeshComponent.SetCustomDataValue` _instancedstaticmesh _index_3 2 1.0 false)
        ;;[1 1 1] Looping [3]
        (`InstancedStaticMeshComponent.SetCustomDataValue` _instancedstaticmesh _index_3 3 1.0 false)
        ;;[1 1 1] TimeStartOffset [4] (rand value)
        (`InstancedStaticMeshComponent.SetCustomDataValue` _instancedstaticmesh _index_3 5 250.0 false)))))