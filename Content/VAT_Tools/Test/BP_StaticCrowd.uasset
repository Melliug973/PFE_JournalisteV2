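; Test actor for a static VAT (vertex animation texture) crowd, laying out a rows-by-columns grid of instances on one InstancedStaticMesh during construction.
; SetRandom picks skeleton, weight class, head and independently rolled outfit pieces from CrowdDataAsset.
; Its results are currently discarded.
; Disconnected nodes would set the mesh and write animation frames, play rate, looping and time offset into per-instance custom data.
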(fn `SetRandom`
  (returns (Face :type "StaticMesh Object Reference") (Top :type "StaticMesh Object Reference") (Body :type "StaticMesh Object Reference") (Bottom :type "StaticMesh Object Reference") (Shoes :type "StaticMesh Object Reference"))
  (bind _returnvalue (`KismetMathLibrary.RandomIntegerInRange` 0 2))
  (bind _crowddataasset (`self.CrowdDataAsset`))
  (bind (_normalweight _overweight _underweight) (break `/Game/CitySampleCrowd/Character/Shared/Structs/CrowdSkeletonDefinition` (`/Game/CitySampleCrowd/Blueprints/BP_CrowdCharacterDataAsset.Skeleton B` _crowddataasset)))
  (bind (_normalweight_2 _overweight_2 _underweight_2) (break `/Game/CitySampleCrowd/Character/Shared/Structs/CrowdSkeletonDefinition` (`/Game/CitySampleCrowd/Blueprints/BP_CrowdCharacterDataAsset.Skeleton A` _crowddataasset)))
  (bind (_body _heads _headsvat _outfits) (break `/Game/CitySampleCrowd/Character/Shared/Structs/CrowdBodyOutfitDefinition` _normalweight_2))
  (bind (_body_2 _heads_2 _headsvat_2 _outfits_2) (break `/Game/CitySampleCrowd/Character/Shared/Structs/CrowdBodyOutfitDefinition` _underweight))
  (bind (_body_3 _heads_3 _headsvat_3 _outfits_3) (break `/Game/CitySampleCrowd/Character/Shared/Structs/CrowdBodyOutfitDefinition` _overweight_2))
  (bind (_body_4 _heads_4 _headsvat_4 _outfits_4) (break `/Game/CitySampleCrowd/Character/Shared/Structs/CrowdBodyOutfitDefinition` _underweight_2))
  (bind (_body_5 _heads_5 _headsvat_5 _outfits_5) (break `/Game/CitySampleCrowd/Character/Shared/Structs/CrowdBodyOutfitDefinition` _normalweight))
  (bind (_body_6 _heads_6 _headsvat_6 _outfits_6) (break `/Game/CitySampleCrowd/Character/Shared/Structs/CrowdBodyOutfitDefinition` _overweight))
  (bind (_top _bottom _shoes _vat_top _vat_bottom _vat_shoes) (break `/Game/CitySampleCrowd/Character/Shared/Structs/CrowdOutfitDefinition` (`|GetArrayItem` _outfits (`KismetMathLibrary.RandomIntegerInRange` 0 12))))
  (bind (_top_2 _bottom_2 _shoes_2 _vat_top_2 _vat_bottom_2 _vat_shoes_2) (break `/Game/CitySampleCrowd/Character/Shared/Structs/CrowdOutfitDefinition` (`|GetArrayItem` _outfits_2 (`KismetMathLibrary.RandomIntegerInRange` 0 14))))
  (bind (_top_3 _bottom_3 _shoes_3 _vat_top_3 _vat_bottom_3 _vat_shoes_3) (break `/Game/CitySampleCrowd/Character/Shared/Structs/CrowdOutfitDefinition` (`|GetArrayItem` _outfits_3 (`KismetMathLibrary.RandomIntegerInRange` 0 12))))
  (bind (_top_4 _bottom_4 _shoes_4 _vat_top_4 _vat_bottom_4 _vat_shoes_4) (break `/Game/CitySampleCrowd/Character/Shared/Structs/CrowdOutfitDefinition` (`|GetArrayItem` _outfits_4 (`KismetMathLibrary.RandomIntegerInRange` 0 12))))
  (bind (_top_5 _bottom_5 _shoes_5 _vat_top_5 _vat_bottom_5 _vat_shoes_5) (break `/Game/CitySampleCrowd/Character/Shared/Structs/CrowdOutfitDefinition` (`|GetArrayItem` _outfits_5 (`KismetMathLibrary.RandomIntegerInRange` 0 14))))
  (bind (_top_6 _bottom_6 _shoes_6 _vat_top_6 _vat_bottom_6 _vat_shoes_6) (break `/Game/CitySampleCrowd/Character/Shared/Structs/CrowdOutfitDefinition` (`|GetArrayItem` _outfits_6 (`KismetMathLibrary.RandomIntegerInRange` 0 14))))
  ;[1 1 1] Select Skeleton type
  (switch `int` (`KismetMathLibrary.RandomIntegerInRange` 0 1)
    (:`0`
      ;[1 1 1] Select Random Weight
      (switch `int` _returnvalue
        (:`0`
          ;[1 1 1] Normal
          (return (`.VAT_69_A233C311492955B380807DAE97AF30C7` (break `/Game/CitySampleCrowd/Character/Shared/Structs/CrowdVATDefinition` (`.VAT_18_BE77C97A448BD4BCCE583A9BFA047B33` (break `/Game/CitySampleCrowd/Character/Shared/Structs/CrowdBodyDefinition` _body)))) (`.VAT_69_A233C311492955B380807DAE97AF30C7` (break `/Game/CitySampleCrowd/Character/Shared/Structs/CrowdVATDefinition` _vat_top)) (`.VAT_69_A233C311492955B380807DAE97AF30C7` (break `/Game/CitySampleCrowd/Character/Shared/Structs/CrowdVATDefinition` (`.VAT_52_7B2E92D3444C784036DD33A01DFA67DD` (break `/Game/CitySampleCrowd/Character/Shared/Structs/CrowdHeadDefinition` (`|GetArrayItem` _headsvat (`KismetMathLibrary.RandomIntegerInRange` 0 5)))))) (`.VAT_69_A233C311492955B380807DAE97AF30C7` (break `/Game/CitySampleCrowd/Character/Shared/Structs/CrowdVATDefinition` _vat_bottom)) (`.VAT_69_A233C311492955B380807DAE97AF30C7` (break `/Game/CitySampleCrowd/Character/Shared/Structs/CrowdVATDefinition` _vat_shoes))))
        (:`1`
          ;[1 1 1] Over
          (return (`.VAT_69_A233C311492955B380807DAE97AF30C7` (break `/Game/CitySampleCrowd/Character/Shared/Structs/CrowdVATDefinition` (`.VAT_52_7B2E92D3444C784036DD33A01DFA67DD` (break `/Game/CitySampleCrowd/Character/Shared/Structs/CrowdHeadDefinition` (`|GetArrayItem` _headsvat_3 (`KismetMathLibrary.RandomIntegerInRange` 0 5)))))) (`.VAT_69_A233C311492955B380807DAE97AF30C7` (break `/Game/CitySampleCrowd/Character/Shared/Structs/CrowdVATDefinition` _vat_top_3)) (`.VAT_69_A233C311492955B380807DAE97AF30C7` (break `/Game/CitySampleCrowd/Character/Shared/Structs/CrowdVATDefinition` (`.VAT_18_BE77C97A448BD4BCCE583A9BFA047B33` (break `/Game/CitySampleCrowd/Character/Shared/Structs/CrowdBodyDefinition` _body_3)))) (`.VAT_69_A233C311492955B380807DAE97AF30C7` (break `/Game/CitySampleCrowd/Character/Shared/Structs/CrowdVATDefinition` _vat_bottom_3)) (`.VAT_69_A233C311492955B380807DAE97AF30C7` (break `/Game/CitySampleCrowd/Character/Shared/Structs/CrowdVATDefinition` _vat_shoes_3))))
        (:`2`
          ;[1 1 1] Under
          (return (`.VAT_69_A233C311492955B380807DAE97AF30C7` (break `/Game/CitySampleCrowd/Character/Shared/Structs/CrowdVATDefinition` (`.VAT_52_7B2E92D3444C784036DD33A01DFA67DD` (break `/Game/CitySampleCrowd/Character/Shared/Structs/CrowdHeadDefinition` (`|GetArrayItem` _headsvat_4 (`KismetMathLibrary.RandomIntegerInRange` 0 5)))))) (`.VAT_69_A233C311492955B380807DAE97AF30C7` (break `/Game/CitySampleCrowd/Character/Shared/Structs/CrowdVATDefinition` _vat_top_4)) (`.VAT_69_A233C311492955B380807DAE97AF30C7` (break `/Game/CitySampleCrowd/Character/Shared/Structs/CrowdVATDefinition` (`.VAT_18_BE77C97A448BD4BCCE583A9BFA047B33` (break `/Game/CitySampleCrowd/Character/Shared/Structs/CrowdBodyDefinition` _body_4)))) (`.VAT_69_A233C311492955B380807DAE97AF30C7` (break `/Game/CitySampleCrowd/Character/Shared/Structs/CrowdVATDefinition` _vat_bottom_4)) (`.VAT_69_A233C311492955B380807DAE97AF30C7` (break `/Game/CitySampleCrowd/Character/Shared/Structs/CrowdVATDefinition` _vat_shoes_4))))))
    (:`1`
      (switch `int` _returnvalue
        (:`0`
          ;[1 1 1] Normal
          (return (`.VAT_69_A233C311492955B380807DAE97AF30C7` (break `/Game/CitySampleCrowd/Character/Shared/Structs/CrowdVATDefinition` (`.VAT_52_7B2E92D3444C784036DD33A01DFA67DD` (break `/Game/CitySampleCrowd/Character/Shared/Structs/CrowdHeadDefinition` (`|GetArrayItem` _headsvat_5 (`KismetMathLibrary.RandomIntegerInRange` 0 5)))))) (`.VAT_69_A233C311492955B380807DAE97AF30C7` (break `/Game/CitySampleCrowd/Character/Shared/Structs/CrowdVATDefinition` _vat_top_5)) (`.VAT_69_A233C311492955B380807DAE97AF30C7` (break `/Game/CitySampleCrowd/Character/Shared/Structs/CrowdVATDefinition` (`.VAT_18_BE77C97A448BD4BCCE583A9BFA047B33` (break `/Game/CitySampleCrowd/Character/Shared/Structs/CrowdBodyDefinition` _body_5)))) (`.VAT_69_A233C311492955B380807DAE97AF30C7` (break `/Game/CitySampleCrowd/Character/Shared/Structs/CrowdVATDefinition` _vat_bottom_5)) (`.VAT_69_A233C311492955B380807DAE97AF30C7` (break `/Game/CitySampleCrowd/Character/Shared/Structs/CrowdVATDefinition` _vat_shoes_5))))
        (:`1`
          ;[1 1 1] Under
          (return (`.VAT_69_A233C311492955B380807DAE97AF30C7` (break `/Game/CitySampleCrowd/Character/Shared/Structs/CrowdVATDefinition` (`.VAT_52_7B2E92D3444C784036DD33A01DFA67DD` (break `/Game/CitySampleCrowd/Character/Shared/Structs/CrowdHeadDefinition` (`|GetArrayItem` _headsvat_2 (`KismetMathLibrary.RandomIntegerInRange` 0 5)))))) (`.VAT_69_A233C311492955B380807DAE97AF30C7` (break `/Game/CitySampleCrowd/Character/Shared/Structs/CrowdVATDefinition` _vat_top_2)) (`.VAT_69_A233C311492955B380807DAE97AF30C7` (break `/Game/CitySampleCrowd/Character/Shared/Structs/CrowdVATDefinition` (`.VAT_18_BE77C97A448BD4BCCE583A9BFA047B33` (break `/Game/CitySampleCrowd/Character/Shared/Structs/CrowdBodyDefinition` _body_2)))) (`.VAT_69_A233C311492955B380807DAE97AF30C7` (break `/Game/CitySampleCrowd/Character/Shared/Structs/CrowdVATDefinition` _vat_bottom_2)) (`.VAT_69_A233C311492955B380807DAE97AF30C7` (break `/Game/CitySampleCrowd/Character/Shared/Structs/CrowdVATDefinition` _vat_shoes_2))))
        (:`2`
          ;[1 1 1] Over
          (return (`.VAT_69_A233C311492955B380807DAE97AF30C7` (break `/Game/CitySampleCrowd/Character/Shared/Structs/CrowdVATDefinition` (`.VAT_52_7B2E92D3444C784036DD33A01DFA67DD` (break `/Game/CitySampleCrowd/Character/Shared/Structs/CrowdHeadDefinition` (`|GetArrayItem` _headsvat_6 (`KismetMathLibrary.RandomIntegerInRange` 0 5)))))) (`.VAT_69_A233C311492955B380807DAE97AF30C7` (break `/Game/CitySampleCrowd/Character/Shared/Structs/CrowdVATDefinition` _vat_top_6)) (`.VAT_69_A233C311492955B380807DAE97AF30C7` (break `/Game/CitySampleCrowd/Character/Shared/Structs/CrowdVATDefinition` (`.VAT_18_BE77C97A448BD4BCCE583A9BFA047B33` (break `/Game/CitySampleCrowd/Character/Shared/Structs/CrowdBodyDefinition` _body_6)))) (`.VAT_69_A233C311492955B380807DAE97AF30C7` (break `/Game/CitySampleCrowd/Character/Shared/Structs/CrowdVATDefinition` _vat_bottom_6)) (`.VAT_69_A233C311492955B380807DAE97AF30C7` (break `/Game/CitySampleCrowd/Character/Shared/Structs/CrowdVATDefinition` _vat_shoes_6))))))))

(fn `UserConstructionScript`
  (for _index (range (`self.Rows`))
    (for _index_2 (range (`self.Columns`))
      (`self.SetRandom`)
      (`InstancedStaticMeshComponent.AddInstance` (`self.InstancedStaticMesh`) (`KismetMathLibrary.MakeTransform` (`KismetMathLibrary.MakeVector` (* _index_2 (`self.ColDistance`)) (* _index (`self.RowDistance`))) (`KismetMathLibrary.MakeRotator` 0.0)) false))))