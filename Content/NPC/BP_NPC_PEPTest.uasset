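; NPC Blueprint variant, named as a test, that switches off inherited interaction elements and can play a cinema voice line.
; After the parent BeginPlay, it hides the interaction text, widget and both spheres in game and disables overlap events on the spheres.
; A custom PlaySon event plays the NPC cinema voice sound at the actor's location with dedicated attenuation.
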(event `self.ReceiveBeginPlay`
  (bind _sphere (`self.Sphere`))
  (`parent.ReceiveBeginPlay`)
  (`SceneComponent.SetVisibility` _sphere true false)
  (`SceneComponent.SetVisibility` (`self.SphereBig`) true false)
  (`SceneComponent.SetVisibility` (`self.TextInteraction`) true false)
  (`SceneComponent.SetVisibility` (`self.Widget`) true false)
  (`SceneComponent.SetHiddenInGame` (`self.Widget`) true false)
  (`SceneComponent.SetHiddenInGame` (`self.TextInteraction`) true false)
  (`SceneComponent.SetHiddenInGame` (`self.SphereBig`) true false)
  (`SceneComponent.SetHiddenInGame` _sphere true false)
  (set `PrimitiveComponent.bGenerateOverlapEvents` false _sphere)
  (set `PrimitiveComponent.bGenerateOverlapEvents` false (`self.SphereBig`)))

(event `PlaySon`
  (`GameplayStatics.PlaySoundAtLocation` (`self.Sound Voice Cinema NPC`) (`self.K2_GetActorLocation`) (struct) 1.0 1.0 0.0 "/Game/DialogueSystem/NPC/CinemaVoiceNPC.CinemaVoiceNPC" null null null))

(fn `UserConstructionScript`
  (`parent.UserConstructionScript`))