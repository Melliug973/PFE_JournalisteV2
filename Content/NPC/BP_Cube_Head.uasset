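; BP_Cube_Head is an NPC head that carries face and name widgets and turns its Sphere toward the player camera every tick.
; BeginPlay creates both widgets, assigns them to their components, and hides these along with the Sphere and Plane.
; PlayAnimationFocus plays a timeline that uniformly scales the face widget, gated by a DoOnce that resets when its condition is false.
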(event `PlayAnimationFocus`
  (params (Condition :type Boolean))
  (bind _widgetface (`self.WidgetFace`))
  (bind (_returnvalue_location _returnvalue_rotation) (`KismetMathLibrary.BreakTransform` (`SceneComponent.K2_GetComponentToWorld` _widgetface)))
  (if Condition
    (`/Engine/EditorBlueprintResources/StandardMacros.DoOnce` false :!label _label
      (:`Completed`
        (bind (_direction _newtrack_0) (`Timeline|Timeline` :!via `PlayFromStart`)
          (:`Update`
            (`SceneComponent.K2_SetWorldTransform` _widgetface (`KismetMathLibrary.MakeTransform` _returnvalue_location _returnvalue_rotation (`KismetMathLibrary.MakeVector` _newtrack_0 _newtrack_0 _newtrack_0)) false false)))))
    (else
      (goto _label :!via `Reset`))))

(event `self.ReceiveTick`
  (params (DeltaSeconds :type "Float (single-precision)"))
  (bind _sphere (`self.Sphere`))
  (`SceneComponent.K2_SetWorldRotation` _sphere (`KismetMathLibrary.FindLookAtRotation` (`SceneComponent.K2_GetComponentLocation` _sphere) (`SceneComponent.K2_GetComponentLocation` (`PlayerCameraManager.TransformComponent` (`GameplayStatics.GetPlayerCameraManager` 0)))) false false))

(event `self.ReceiveBeginPlay`
  (`SceneComponent.SetVisibility` (`self.Sphere`) false false)
  (`SceneComponent.SetVisibility` (`self.WidgetFace`) false false)
  (`SceneComponent.SetVisibility` (`self.Plane`) false false)
  (`SceneComponent.SetVisibility` (`self.WidgetName`) false false)
  (bind _returnvalue (`|CreateWidget` "/Game/NPC/WB_NPCFace.WB_NPCFace_C"))
  (bind _output_get (set `self.WD_Face` _returnvalue))
  (`WidgetComponent.SetWidget` (`self.WidgetFace`) _output_get)
  (bind _returnvalue_2 (`|CreateWidget` "/Game/NPC/WB_Name_NPC.WB_Name_NPC_C"))
  (bind _output_get_2 (set `self.WB Name` _returnvalue_2))
  (`WidgetComponent.SetWidget` (`self.WidgetName`) _output_get_2))

(fn `UserConstructionScript`)