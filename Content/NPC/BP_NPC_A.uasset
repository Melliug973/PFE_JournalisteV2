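; NPC actor that shows an interaction prompt and turns to face the player when approached.
; Entering SphereBig reveals the widget and text and enables the inner Sphere, then hides and disables them after a delay or on exit.
; Overlapping Sphere with the third-person character starts a looping timer that smoothly interpolates yaw toward them, cleared on exit.
; SetVisibilityWidget toggles the prompt while disabling both trigger spheres.
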(event `self.ReceiveBeginPlay`
  (bind _widget (`self.Widget`))
  (bind _spherebig (`self.SphereBig`))
  (`SceneComponent.SetVisibility` (`self.TAG`) true false)
  (`SceneComponent.SetVisibility` (`self.Sphere`) false false)
  (set `PrimitiveComponent.bGenerateOverlapEvents` false (`self.Sphere`))
  (`SceneComponent.SetVisibility` _widget false false)
  (`SceneComponent.SetVisibility` (`self.TextInteraction`) false false)
  (set `PrimitiveComponent.bGenerateOverlapEvents` false (`self.TextInteraction`))
  (set `PrimitiveComponent.bGenerateOverlapEvents` false _widget)
  (`SceneComponent.SetVisibility` _spherebig true false)
  (set `PrimitiveComponent.bGenerateOverlapEvents` true _spherebig))

(event `SetVisibilityWidget`
  (params (bNewVisibility :type Boolean))
  (bind _sphere (`self.Sphere`))
  (`SceneComponent.SetVisibility` (`self.Widget`) bNewVisibility false)
  (`SceneComponent.SetVisibility` (`self.TextInteraction`) bNewVisibility false)
  (`SceneComponent.SetVisibility` _sphere false false)
  (`SceneComponent.SetVisibility` (`self.SphereBig`) false false)
  (set `PrimitiveComponent.bGenerateOverlapEvents` false _sphere)
  (set `PrimitiveComponent.bGenerateOverlapEvents` false (`self.SphereBig`)))

(event `self.SphereBig.OnComponentBeginOverlap`
  (params (OverlappedComponent :type "PrimitiveComponent Object Reference") (OtherActor :type "Actor Object Reference") (OtherComp :type "PrimitiveComponent Object Reference") (OtherBodyIndex :type Integer) (bFromSweep :type Boolean) (SweepResult :type "HitResult Structure (by ref)"))
  (bind _sphere (`self.Sphere`))
  (bind _widget (`self.Widget`))
  (`SceneComponent.SetVisibility` (`self.SphereBig`) false false)
  (set `self.CharacterOnClose` true)
  (`SceneComponent.SetVisibility` _sphere true false)
  (set `PrimitiveComponent.bGenerateOverlapEvents` true _sphere)
  (`SceneComponent.SetVisibility` _widget true false)
  (`SceneComponent.SetVisibility` (`self.TextInteraction`) true false)
  (`KismetSystemLibrary.Delay` 2.0)
  (set `self.CharacterOnClose` false :!label _label)
  (set `PrimitiveComponent.bGenerateOverlapEvents` false (`self.Sphere`))
  (`SceneComponent.SetVisibility` _widget false false)
  (`SceneComponent.SetVisibility` (`self.TextInteraction`) false false)
  (`SceneComponent.SetVisibility` (`self.Sphere`) false false)
  (`PrimitiveComponent.SetCollisionEnabled` _widget "NoCollision")
  (`PrimitiveComponent.SetCollisionEnabled` (`self.TextInteraction`) "NoCollision"))

(event `self.SphereBig.OnComponentEndOverlap`
  (params (OverlappedComponent :type "PrimitiveComponent Object Reference") (OtherActor :type "Actor Object Reference") (OtherComp :type "PrimitiveComponent Object Reference") (OtherBodyIndex :type Integer))
  (goto _label))

(event `self.Sphere.OnComponentBeginOverlap`
  (params (OverlappedComponent :type "PrimitiveComponent Object Reference") (OtherActor :type "Actor Object Reference") (OtherComp :type "PrimitiveComponent Object Reference") (OtherBodyIndex :type Integer) (bFromSweep :type Boolean) (SweepResult :type "HitResult Structure (by ref)"))
  (set `self.CharacterOnClose` true)
  (bind _asbp_third_person_character (cast `/Game/ThirdPerson/Blueprints/BP_ThirdPersonCharacter` OtherActor))
  (set `self.As BP Third Person Character` _asbp_third_person_character)
  (bind _returnvalue (`KismetSystemLibrary.K2_SetTimerDelegate` (delegate `Rotate`) 0.01 true))
  (set `self.Timer Handle` _returnvalue)
  (`SceneComponent.SetVisibility` (`self.SphereBig`) false false)
  (set `PrimitiveComponent.bGenerateOverlapEvents` true (`self.Sphere`))
  (`SceneComponent.SetVisibility` (`self.Widget`) true false)
  (`SceneComponent.SetVisibility` (`self.TextInteraction`) true false))

(event `Rotate`
  (bind (_returnvalue_roll _returnvalue_pitch _returnvalue_yaw) (`KismetMathLibrary.BreakRotator` (`KismetMathLibrary.RInterpTo` (`self.K2_GetActorRotation`) (`KismetMathLibrary.FindLookAtRotation` (`self.K2_GetActorLocation`) (`self.K2_GetActorLocation` (`self.As BP Third Person Character`))) (`GameplayStatics.GetWorldDeltaSeconds`) 1.0)))
  (`self.K2_SetActorRotation` (`KismetMathLibrary.MakeRotator` 0.0 0.0 _returnvalue_yaw)))

(event `self.Sphere.OnComponentEndOverlap`
  (params (OverlappedComponent :type "PrimitiveComponent Object Reference") (OtherActor :type "Actor Object Reference") (OtherComp :type "PrimitiveComponent Object Reference") (OtherBodyIndex :type Integer))
  (bind _widget (`self.Widget`))
  (`KismetSystemLibrary.K2_ClearAndInvalidateTimerHandle` (`self.Timer Handle`))
  (`SceneComponent.SetVisibility` (`self.SphereBig`) true false)
  (set `self.CharacterOnClose` false)
  (`SceneComponent.SetVisibility` _widget false false)
  (`SceneComponent.SetVisibility` (`self.TextInteraction`) false false)
  (`PrimitiveComponent.SetCollisionEnabled` _widget "NoCollision")
  (`PrimitiveComponent.SetCollisionEnabled` (`self.TextInteraction`) "NoCollision"))

(fn `UserConstructionScript`)