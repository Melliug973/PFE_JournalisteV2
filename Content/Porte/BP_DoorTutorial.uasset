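; Tutorial door actor that registers itself with the NPC_Tutorial character and tracks when the player is within range.
; A box collision, also checked shortly after BeginPlay, passes the door to the NPC and sets an OpenDoor flag for the player, clearing both on exit.
; Separate events toggle door and handle collision, store a right-hand reference, and swing the door root's yaw through in and out timelines.
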(event `self.ReceiveBeginPlay`
  (`|ExecutionSequence`
    (:`then_0`
      (bind _returnvalue (`GameplayStatics.GetActorOfClass` "/Game/NPC/Tutorial/NPC_Tutorial.NPC_Tutorial_C"))
      (set `self.NPC` _returnvalue)
      (`KismetSystemLibrary.Delay` 0.2)
      (`self.Is Overlap Door`))
    (:`then_1`
      (bind _asbp_third_person_character (cast `/Game/ThirdPerson/Blueprints/BP_ThirdPersonCharacter` (`GameplayStatics.GetPlayerCharacter` 0)))
      (set `self.As BP Third Person Character_0` _asbp_third_person_character))))

(event `Is Overlap Door`
  (for _array_element (`PrimitiveComponent.GetOverlappingActors` (`self.BoxCollision`) null)
    (if (== _array_element (`self.NPC`))
      (message `/Game/Porte/Blueprint/Interface/BPI_Door.SetNewDoorTutorial` _array_element self))))

(event `AttachRightMouse`
  (params (`Right Hand` :type Boolean))
  (set `self.Right Hand` `Right Hand`))

(event `self.BoxCollision.OnComponentBeginOverlap`
  (params (OverlappedComponent :type "PrimitiveComponent Object Reference") (OtherActor :type "Actor Object Reference") (OtherComp :type "PrimitiveComponent Object Reference") (OtherBodyIndex :type Integer) (bFromSweep :type Boolean) (SweepResult :type "HitResult Structure (by ref)"))
  (`|ExecutionSequence`
    (:`then_0`
      (if (== OtherActor (`self.NPC`))
        (message `/Game/Porte/Blueprint/Interface/BPI_Door.SetNewDoorTutorial` OtherActor self)))
    (:`then_1`
      (if (== OtherActor (`self.As BP Third Person Character_0`))
        (set `self.OpenDoor?` true)
        (`KismetSystemLibrary.PrintString` (`KismetStringLibrary.Conv_BoolToString` (`self.OpenDoor?`)))))))

(event `self.BoxCollision.OnComponentEndOverlap`
  (params (OverlappedComponent :type "PrimitiveComponent Object Reference") (OtherActor :type "Actor Object Reference") (OtherComp :type "PrimitiveComponent Object Reference") (OtherBodyIndex :type Integer))
  (message `/Game/Porte/Blueprint/Interface/BPI_Door.SetNewDoorTutorial` OtherActor null)
  (set `self.OpenDoor?` false))

(event `SetCollisionDoor`
  (params (Collision :type Boolean))
  (if Collision
    (`PrimitiveComponent.SetCollisionEnabled` (`self.Door`) "QueryAndPhysics")
    (`PrimitiveComponent.SetCollisionEnabled` (`self.Handle1`) "QueryAndPhysics")
    (`PrimitiveComponent.SetCollisionEnabled` (`self.Handle`) "QueryAndPhysics")
    (else
      (`PrimitiveComponent.SetCollisionEnabled` (`self.Door`) "NoCollision")
      (`PrimitiveComponent.SetCollisionEnabled` (`self.Handle1`) "NoCollision")
      (`PrimitiveComponent.SetCollisionEnabled` (`self.Handle`) "NoCollision"))))

(event `Rotate Door In`
  (bind (_direction _zrotation) (`Timeline|Door Rotate In` :!via `PlayFromStart`)
    (:`Update`
      (`SceneComponent.K2_SetRelativeRotation` (`self.DoorRoot`) (`KismetMathLibrary.MakeRotator` 0.0 0.0 (* _zrotation -90.0)) false false))))

(event `Rotate Door Out`
  (bind (_direction _zrotation) (`Timeline|Timeline`)
    (:`Update`
      (`SceneComponent.K2_SetRelativeRotation` (`self.DoorRoot`) (`KismetMathLibrary.MakeRotator` 0.0 0.0 (* _zrotation -90.0)) false false))))

(fn `UserConstructionScript`)