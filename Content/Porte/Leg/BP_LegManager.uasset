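; Actor component on NPC_20022 that manages the character's two procedural legs and coordinates their stepping.
; On BeginPlay it caches the owner's left and right leg references, then calls UpdateFoot on each every Tick.
; CanLegUnplant allows a leg to lift only while another leg is planted, and GetLegReference returns a leg by tag.
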(event `self.ReceiveBeginPlay`
  (`self.Get ComponentReference`))

(event `self.ReceiveTick`
  (params (DeltaSeconds :type "Float (single-precision)"))
  (`self.UpdateAllLegs`))

(event `UpdateAllLegs`
  (for _array_element (`self.Legs`)
    (`/Game/Porte/Leg/BP_Leg.UpdateFoot` _array_element)))

(fn `CanLegUnplant`
  (params (Leg :type "/Game/Porte/Leg/BP_Leg Object Reference"))
  (returns (`Can Unplant` :type Boolean))
  (for _array_element (`self.Legs`)
    (if (and (`/Game/Porte/Leg/BP_Leg.IsPlanted` _array_element) (!= _array_element Leg))
      (return true)))
  (return false))

(fn `Get ComponentReference`
  (bind _legs (`self.Legs`))
  (bind _asnpc_20022 (cast `/Game/Porte/NPC/NPC_20022` (`self.GetOwner`)))
  (`KismetArrayLibrary.Array_Add` _legs (`/Game/Porte/NPC/NPC_20022.BP_Leg_Left` _asnpc_20022))
  (`KismetArrayLibrary.Array_Add` _legs (`/Game/Porte/NPC/NPC_20022.BP_Leg_Right` _asnpc_20022))
  (return))

(fn `GetLegReference`
  (params (LegTag :type String))
  (returns (OutLeg :type "/Game/Porte/Leg/BP_Leg Object Reference"))
  (bind _asnpc_20022 (cast `/Game/Porte/NPC/NPC_20022` (`self.GetOwner`)))
  (switch `string` LegTag
    (:`LeftLeg`
      (return (`/Game/Porte/NPC/NPC_20022.BP_Leg_Left` _asnpc_20022)))
    (:`RightLeg`
      (return (`/Game/Porte/NPC/NPC_20022.BP_Leg_Right` _asnpc_20022)))))