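; Procedural leg component for NPC_20022 that finds ground footholds and animates the foot stepping between them.
; UpdateFoot traces along the component's forward vector, falling back to a downward trace from the ray end.
; When the planted foot drifts too far from the target and LegManager permits, it steps there using speed and height curves.
; Unplant and replant changes are messaged to the NPC's AnimInstance.
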(event `self.ReceiveBeginPlay`
  (set `self.Foot Position` (`self.K2_GetComponentLocation`))
  (bind _returnvalue (`GameplayStatics.GetActorOfClass` "/Game/Porte/NPC/NPC_20022.NPC_20022_C"))
  (set `self.NPC` _returnvalue)
  (set `self.AnimInstance` (`SkeletalMeshComponent.GetAnimInstance` (`Character.Mesh` (`self.NPC`)))))

(event `SetDefaultPosition`
  (bind _trace_position (`self.Trace Position`))
  (`self.GetFootTargetLocation`)
  (set `self.Plant Start Position` _trace_position)
  (set `self.Target Position` _trace_position)
  (set `self.Foot Position` _trace_position)
  (set `self.IsPlanted` true))

(fn `CheckForReplant`
  (`|ExecutionSequence`
    (:`then_0`
      (set `self.Want To Replant` (and (`self.IsPlanted`) (> (`KismetMathLibrary.VSize` (- (`self.Foot Position`) (`self.Target Position`))) (`self.Stop Distance`)))))
    (:`then_1`
      (set `self.Do Replant` (and (`self.Want To Replant`) (`/Game/Porte/Leg/BP_LegManager.CanLegUnplant` (`self.Leg Manager`) self))))
    (:`then_2`
      (if (`self.Do Replant`)
        (`|ExecutionSequence`
          (:`then_0`
            (set `self.IsPlanted` false)
            (message `/Game/Porte/Blueprint/Interface/BPI_Anim.SetUnplanted` (`self.AnimInstance`) self false))
          (:`then_1`
            (set `self.Plant Start Position` (`self.Foot Position`)))
          (:`then_2`
            (set `self.Time Since Unplanted` 0.0)))))))

(fn `DebugDraw`
  (`KismetSystemLibrary.DrawDebugSphere` (`self.Foot Position`) 4.0 12 (struct :`R` 0.089607 :`G` 1.0 :`A` 1.0) 0.0 2.0))

(fn `GetFootTargetLocation`
  (bind _ray_end (`self.Ray End`))
  (`|ExecutionSequence`
    (:`then_0`
      (set `self.Ray Start` (`self.K2_GetComponentLocation`)))
    (:`then_1`
      (set `self.Ray End` (+ (`self.Ray Start`) (* (`KismetMathLibrary.GetForwardVector` (.rotation (`self.K2_GetComponentToWorld`))) (`self.Ray Cast Length`)))))
    (:`then_2`
      (bind _location (`self.Cast Ray` (`self.Ray Start`) (`self.Ray End`))
        (:`True`
          (set `self.Trace Position` _location))
        (:`False`
          (bind _location_2 (`self.Cast Ray` _ray_end (- _ray_end (`KismetMathLibrary.MakeVector` 0.0 0.0 (* (`self.Ray Cast Length`) 4.0))))
            (:`True`
              (set `self.Trace Position` _location_2))
            (:`False`
              (set `self.Trace Position` (`self.Target Position`)))))))
    (:`then_3`
      (set `self.Target Position` (`self.Trace Position`)))))

(fn `TakeFootstep`
  (if (not (`self.IsPlanted`))
    (`|ExecutionSequence`
      (:`then_0`
        (set `self.Percentage Replanted` (/ (`self.Time Since Unplanted`) (`self.Stop Time`))))
      (:`then_1`
        (set `self.Foot Position No Height` (`KismetMathLibrary.VLerp` (`self.Plant Start Position`) (`self.Target Position`) (`CurveFloat.GetFloatValue` (`self.Replant Speed Curve`) (`self.Percentage Replanted`)))))
      (:`then_2`
        (set `self.Foot Position` (+ (`self.Foot Position No Height`) (`KismetMathLibrary.MakeVector` 0.0 0.0 (* (`CurveFloat.GetFloatValue` (`self.Replant Height Curve`) (`self.Percentage Replanted`)) (`self.Stop Height`))))))
      (:`then_3`
        (set `self.Time Since Unplanted` (+ (`self.Time Since Unplanted`) (`GameplayStatics.GetWorldDeltaSeconds`)))
        (bind _output_get (set `self.IsPlanted` (>= (`self.Time Since Unplanted`) (`self.Stop Time`))))
        (if _output_get
          (message `/Game/Porte/Blueprint/Interface/BPI_Anim.SetUnplanted` (`self.AnimInstance`) self true))))))

(fn `UpdateFoot`
  (`self.GetFootTargetLocation`)
  (`self.CheckForReplant`)
  (`self.TakeFootstep`)
  (if (`self.Debug Draw`)
    (`self.DebugDraw`)))