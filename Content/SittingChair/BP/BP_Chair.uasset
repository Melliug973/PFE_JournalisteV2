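; Interactable chair actor that lets a character sit down and stand up, extending its parent's interaction events.
; StartInteraction disables the interacting character's movement through a message call, plays a sitting montage and uses MoveComponentTo to glide the capsule onto the chair, aligned to its yaw.
; EndInteraction stops the montage, moves the character to the StandLocation component and re-enables movement, with CharacterOnChair tracking occupancy.
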(event `self.ReceiveBeginPlay`
  (`parent.ReceiveBeginPlay`)
  (bind _asbp_third_person_character (cast `/Game/ThirdPerson/Blueprints/BP_ThirdPersonCharacter` (`GameplayStatics.GetPlayerCharacter` 0)))
  (set `self.As BP Third Person Character` _asbp_third_person_character))

(event `self.StartInteraction`
  (bind (_returnvalue_roll _returnvalue_pitch _returnvalue_yaw) (`KismetMathLibrary.BreakRotator` (`self.K2_GetActorRotation`)))
  (bind _as_character (`self.As Character`))
  (`parent.StartInteraction`)
  (bind _ascharacter (cast `Character` (`self.InteractingActor`)))
  (bind _output_get (set `self.As Character` _ascharacter))
  (message `/Game/SittingChair/BP/BPI_Character.ToggleMovement` _output_get false)
  (`Character.PlayAnimMontage` _output_get "/Game/SittingChair/Animation/SittingIdle_UE_Montage.SittingIdle_UE_Montage" 1.0 "None")
  (`KismetSystemLibrary.MoveComponentTo` (`Actor.RootComponent` _as_character) (+ (`self.K2_GetActorLocation`) (`KismetMathLibrary.MakeVector` 0.0 0.0 (`CapsuleComponent.CapsuleHalfHeight` (`Character.CapsuleComponent` _as_character)))) (`KismetMathLibrary.MakeRotator` 0.0 0.0 _returnvalue_yaw) false false 0.5)
  (set `self.CharacterOnChair?` true))

(event `self.EndInteraction`
  (bind _as_character (`self.As Character`))
  (`parent.EndInteraction`)
  (bind _as_character_2 (`self.As Character`)
    (:`then`
      (`Character.StopAnimMontage` _as_character_2 "/Game/SittingChair/Animation/SittingIdle_UE_Montage.SittingIdle_UE_Montage")
      (`KismetSystemLibrary.MoveComponentTo` (`Actor.RootComponent` _as_character) (+ (`KismetMathLibrary.MakeVector` 0.0 0.0 (`CapsuleComponent.CapsuleHalfHeight` (`Character.CapsuleComponent` _as_character))) (`SceneComponent.K2_GetComponentLocation` (`self.StandLocation`))) (`self.K2_GetActorRotation` _as_character))
      (message `/Game/SittingChair/BP/BPI_Character.ToggleMovement` (`self.As Character`) true)
      (set `self.CharacterOnChair?` false))
    (:`else`)))

(fn `UserConstructionScript`
  (`parent.UserConstructionScript`))