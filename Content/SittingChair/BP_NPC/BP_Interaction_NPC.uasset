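; BP_Interaction_NPC is a box-trigger actor that tracks when an NPC is interacting with it.
; On begin overlap, an IsNPCMessage check filters for NPCs, stores the InteractingActor and calls StartInteractionNPC to set the Interacting flag.
; Any end overlap clears the stored actor and calls EndInteractionNPC to reset the flag, without checking which actor left.
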(event `self.Box.OnComponentBeginOverlap`
  (params (OverlappedComponent :type "PrimitiveComponent Object Reference") (OtherActor :type "Actor Object Reference") (OtherComp :type "PrimitiveComponent Object Reference") (OtherBodyIndex :type Integer) (bFromSweep :type Boolean) (SweepResult :type "HitResult Structure (by ref)"))
  (bind _yes_no (message `/Game/SittingChair/BP_NPC/BPI_NPC.IsNPC?` OtherActor))
  (if _yes_no
    (`/Engine/EditorBlueprintResources/StandardMacros.IsValid` OtherActor
      (:`Is Valid`
        (set `self.InteractingActor` OtherActor)
        (`self.StartInteractionNPC`)))))

(event `self.Box.OnComponentEndOverlap`
  (params (OverlappedComponent :type "PrimitiveComponent Object Reference") (OtherActor :type "Actor Object Reference") (OtherComp :type "PrimitiveComponent Object Reference") (OtherBodyIndex :type Integer))
  (set `self.InteractingActor` null)
  (`self.EndInteractionNPC`))

(event `StartInteractionNPC`
  (set `self.Interacting` true))

(event `EndInteractionNPC`
  (set `self.Interacting` false))

(fn `UserConstructionScript`)