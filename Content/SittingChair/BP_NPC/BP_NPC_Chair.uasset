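; Chair actor that seats the tutorial NPC when it walks into the chair's trigger box.
; The box starts with collision off, and Tick enables it while the NPC's SittingTrue flag is set.
; On overlap, the NPC plays a sitting montage, moves onto the chair with MoveComponentTo and gets flagged as seated.
; Stand-up logic toward a StandLocation exists but is disconnected.
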(event `self.ReceiveBeginPlay`
  (bind _returnvalue (`GameplayStatics.GetActorOfClass` "/Game/NPC/Tutorial/NPC_Tutorial.NPC_Tutorial_C"))
  (set `self.NPC` _returnvalue)
  (`PrimitiveComponent.SetCollisionEnabled` (`self.Box`) "NoCollision"))

(event `self.ReceiveTick`
  (params (DeltaSeconds :type "Float (single-precision)"))
  (if (`/Game/NPC/Tutorial/NPC_Tutorial.SittingTrue?` (`self.NPC`))
    (`PrimitiveComponent.SetCollisionEnabled` (`self.Box`) "QueryAndPhysics")))

(event `self.Box.OnComponentBeginOverlap`
  (params (OverlappedComponent :type "PrimitiveComponent Object Reference") (OtherActor :type "Actor Object Reference") (OtherComp :type "PrimitiveComponent Object Reference") (OtherBodyIndex :type Integer) (bFromSweep :type Boolean) (SweepResult :type "HitResult Structure (by ref)"))
  (bind (_returnvalue_roll _returnvalue_pitch _returnvalue_yaw) (`KismetMathLibrary.BreakRotator` (`self.K2_GetActorRotation`)))
  (bind _npc (`self.NPC`))
  (bind _npc_2 (`self.NPC`))
  (if (== OtherActor _npc)
    (`Character.PlayAnimMontage` _npc "/Game/SittingChair/AnimationNPC/SittingIdle_UE_Montage.SittingIdle_UE_Montage" 1.0 "None")
    (`KismetSystemLibrary.MoveComponentTo` (`Actor.RootComponent` _npc_2) (+ (`self.K2_GetActorLocation`) (`KismetMathLibrary.MakeVector` 0.0 0.0 (`CapsuleComponent.CapsuleHalfHeight` (`Character.CapsuleComponent` _npc_2)))) (`KismetMathLibrary.MakeRotator` 0.0 0.0 _returnvalue_yaw) false false 0.5)
    (set `/Game/NPC/Tutorial/NPC_Tutorial.NPCOnChair?` true (`self.NPC`))))

(event `self.Box.OnComponentEndOverlap`
  (params (OverlappedComponent :type "PrimitiveComponent Object Reference") (OtherActor :type "Actor Object Reference") (OtherComp :type "PrimitiveComponent Object Reference") (OtherBodyIndex :type Integer)))

(fn `UserConstructionScript`)