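; Interactable chair that seats an NPC_Tutorial character and stands it back up through the parent's NPC interaction events.
; On start, it casts and stores the interacting actor, plays the sitting idle montage and glides its root onto the chair's position and yaw with MoveComponentTo.
; On end, it stops the montage and moves the NPC to StandLocation, offsetting by capsule half-height both ways and tracking occupancy in NPCOnChair.
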(event `self.StartInteractionNPC`
  (bind (_returnvalue_roll _returnvalue_pitch _returnvalue_yaw) (`KismetMathLibrary.BreakRotator` (`self.K2_GetActorRotation`)))
  (bind _as_npc_tutorial (`self.As NPC Tutorial`))
  (`parent.StartInteractionNPC`)
  (bind _asnpc_tutorial (cast `/Game/NPC/Tutorial/NPC_Tutorial` (`self.InteractingActor`)))
  (bind _output_get (set `self.As NPC Tutorial` _asnpc_tutorial))
  (`Character.PlayAnimMontage` _output_get "/Game/SittingChair/AnimationNPC/SittingIdle_UE_Montage.SittingIdle_UE_Montage" 1.0 "None")
  (`KismetSystemLibrary.MoveComponentTo` (`Actor.RootComponent` _as_npc_tutorial) (+ (`self.K2_GetActorLocation`) (`KismetMathLibrary.MakeVector` 0.0 0.0 (`CapsuleComponent.CapsuleHalfHeight` (`Character.CapsuleComponent` _as_npc_tutorial)))) (`KismetMathLibrary.MakeRotator` 0.0 0.0 _returnvalue_yaw) false false 0.5)
  (set `self.NPCOnChair?` true))

(event `self.EndInteractionNPC`
  (bind _as_npc_tutorial (`self.As NPC Tutorial`))
  (`parent.EndInteractionNPC`)
  (bind _as_npc_tutorial_2 (`self.As NPC Tutorial`)
    (:`then`
      (`Character.StopAnimMontage` _as_npc_tutorial_2 "/Game/SittingChair/AnimationNPC/SittingIdle_UE_Montage.SittingIdle_UE_Montage")
      (`KismetSystemLibrary.MoveComponentTo` (`Actor.RootComponent` _as_npc_tutorial) (+ (`KismetMathLibrary.MakeVector` 0.0 0.0 (`CapsuleComponent.CapsuleHalfHeight` (`Character.CapsuleComponent` _as_npc_tutorial))) (`SceneComponent.K2_GetComponentLocation` (`self.StandLocation`))) (`self.K2_GetActorRotation` _as_npc_tutorial))
      (set `self.NPCOnChair?` false))
    (:`else`)))

(fn `UserConstructionScript`
  (`parent.UserConstructionScript`))