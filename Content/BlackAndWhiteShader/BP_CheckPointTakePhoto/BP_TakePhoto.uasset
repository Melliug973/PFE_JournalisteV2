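; Photo-objective checkpoint that makes the player take a picture, with a waypoint widget showing distance to it.
; Box overlap calls ColorScreen, disables player movement, opens the camera and sets stop flags.
; Tick hides the markers while the player is in black-and-white, updates distance and, for Obj1, checks for two tags, Civil and Vigile in either order, then releases the player and destroys the actor.
; Obj2 is empty, and the plane-scale and particle-toggle chains are unconnected.
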(event `self.ReceiveBeginPlay`
  (bind _asbp_third_person_character (cast `/Game/ThirdPerson/Blueprints/BP_ThirdPersonCharacter` (`GameplayStatics.GetPlayerCharacter` 0)))
  (set `self.As BP Third Person Character` _asbp_third_person_character)
  (bind _aswd_waypoint (cast `/Game/BlackAndWhiteShader/Widget/WD_Waypoint` (`WidgetComponent.GetWidget` (`self.Waypoint`))))
  (set `self.As WD Waypoint` _aswd_waypoint)
  (set `self.Distance Text ` (`/Game/BlackAndWhiteShader/Widget/WD_Waypoint.DistanceText` (`self.As WD Waypoint`))))

(event `self.Box.OnComponentBeginOverlap`
  (params (OverlappedComponent :type "PrimitiveComponent Object Reference") (OtherActor :type "Actor Object Reference") (OtherComp :type "PrimitiveComponent Object Reference") (OtherBodyIndex :type Integer) (bFromSweep :type Boolean) (SweepResult :type "HitResult Structure (by ref)"))
  (bind _as_bp_third_person_character (`self.As BP Third Person Character`))
  (`KismetSystemLibrary.PrintString` "Hello")
  (`/Game/ThirdPerson/Blueprints/BP_ThirdPersonCharacter.ColorScreen` _as_bp_third_person_character)
  (`/Game/ThirdPerson/Blueprints/BP_ThirdPersonCharacter.ToggleMovement` _as_bp_third_person_character false true)
  (`/Game/ThirdPerson/Blueprints/BP_ThirdPersonCharacter.OpenCamera` _as_bp_third_person_character)
  (set `/Game/ThirdPerson/Blueprints/BP_ThirdPersonCharacter.StopTakePhoto` true _as_bp_third_person_character)
  (set `/Game/ThirdPerson/Blueprints/BP_ThirdPersonCharacter.StopOpenAplication` true _as_bp_third_person_character))

(event `self.ReceiveTick`
  (params (DeltaSeconds :type "Float (single-precision)"))
  (bind _as_bp_third_person_character (`self.As BP Third Person Character`))
  (bind _waypoint (`self.Waypoint`))
  (bind _as_bp_third_person_character_2 (`self.As BP Third Person Character`))
  (bind _listtag (`/Game/ThirdPerson/Blueprints/BP_ThirdPersonCharacter.ListTag` _as_bp_third_person_character))
  (`|ExecutionSequence`
    (:`then_0`
      (if (== (`/Game/ThirdPerson/Blueprints/BP_ThirdPersonCharacter.IsBlackAndWhite?` _as_bp_third_person_character) true)
        (`SceneComponent.SetVisibility` _waypoint false false)
        (`SceneComponent.SetVisibility` (`self.ParticleSystem`) false false)
        (`SceneComponent.SetVisibility` (`self.Plane`) false false)
        (else
          (`SceneComponent.SetVisibility` _waypoint true false)
          (`SceneComponent.SetVisibility` (`self.ParticleSystem`) true false)
          (`SceneComponent.SetVisibility` (`self.Plane`) true false))))
    (:`then_1`
      (if (`self.Obj1`)
        (if (== (`KismetArrayLibrary.Array_Length` _listtag) 2)
          (for (_array_element _array_index) _listtag
            (`|ExecutionSequence`
              (:`then_0`
                (if (== _array_index 0)
                  (bind _returnvalue (`KismetStringLibrary.Conv_StringToName` _array_element))
                  (if (== _returnvalue "Civil")
                    (set `self.Ind0Civil` true)
                    (else
                      (set `self.Ind0Civil` false)
                      (if (== _returnvalue "Vigile")
                        (set `self.Ind0Vigile` true)
                        (else
                          (set `self.Ind0Vigile` false)))))))
              (:`then_1`
                (if (== _array_index 1)
                  (bind _returnvalue_2 (`KismetStringLibrary.Conv_StringToName` _array_element))
                  (if (== _returnvalue_2 "Civil")
                    (set `self.Ind1Civil` true)
                    (else
                      (set `self.Ind1Civil` false)
                      (if (== _returnvalue_2 "Vigile")
                        (set `self.Ind1Vigile` true)
                        (else
                          (set `self.Ind1Vigile` false)))))))))
          (if (or (and (== (`self.Ind0Civil`) true) (== (`self.Ind1Vigile`) true)) (and (== (`self.Ind1Civil`) true) (== (`self.Ind0Vigile`) true)))
            (`/Game/ThirdPerson/Blueprints/BP_ThirdPersonCharacter.ToggleMovement` _as_bp_third_person_character_2 true true)
            (set `/Game/ThirdPerson/Blueprints/BP_ThirdPersonCharacter.StopTakePhoto` false _as_bp_third_person_character_2)
            (set `/Game/ThirdPerson/Blueprints/BP_ThirdPersonCharacter.StopOpenAplication` false _as_bp_third_person_character_2)
            (`self.K2_DestroyActor`)))))
    (:`then_2`
      (if (`self.Obj2`)
        _))
    (:`then_3`
      (`TextBlock.SetText` (`self.Distance Text `) (`KismetTextLibrary.Conv_StringToText` (`KismetStringLibrary.Concat_StrStr` (`KismetStringLibrary.Conv_IntToString` (`KismetMathLibrary.FTrunc` (/ (`KismetMathLibrary.Vector_Distance` (`self.K2_GetActorLocation`) (`self.K2_GetActorLocation` (`GameplayStatics.GetPlayerPawn` 0))) 100.0))) "m"))))))

(fn `UserConstructionScript`)