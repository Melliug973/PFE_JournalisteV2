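; Poolable car actor for Mass AI traffic, built around a MassTrafficVehicle component.
; The construction script registers the four wheel meshes with that component and writes packed traffic custom data to the body's primitive data.
; It also gives the body a dynamic car-paint material with one of five random colors.
; Pooling is always allowed; the pooling and Tick events are empty, and the wheel-spin experiments are disconnected.
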(event `self.ReceiveTick`
  (params (DeltaSeconds :type "Float (single-precision)")))

(event `MassActorPoolableInterface.PrepareForPooling`)

(event `MassActorPoolableInterface.PrepareForGame`)

(fn `CanBePooled`
  (returns (ReturnValue :type Boolean))
  (return true))

(fn `UserConstructionScript`
  (bind _body (`self.Body`))
  (set `MassTrafficVehicleComponent.WheelComponents` (`|MakeArray` (`self.WheelFL`) (`self.WheelFR`) (`self.WheelRL`) (`self.WheelRR`) :!type "SceneComponent Object Reference") (`self.MassTrafficVehicle`))
  (`PrimitiveComponent.SetCustomPrimitiveDataFloat` _body 1 (`.PackedParam1` (break `MassTrafficPackedVehicleInstanceCustomData` (`MassTrafficFunctionLibrary.GetPackedTrafficVehicleInstanceCustomData` _body))))
  (bind _returnvalue (`PrimitiveComponent.CreateDynamicMaterialInstance` (`self.Body`) 0 "/Game/Megascans/3D_Assets/Car/MI_CarPaint.MI_CarPaint" "None"))
  (`MaterialInstanceDynamic.SetVectorParameterValue` _returnvalue "PaintColor" (select `int` (`KismetMathLibrary.RandomIntegerInRange` 0 4) :`0` (struct :`R` 0.005182 :`G` 0.048172 :`B` 0.07036 :`A` 1.0) :`1` (struct :`R` 0.07036 :`G` 0.007499 :`B` 0.006512 :`A` 1.0) :`2` (struct :`R` 0.052861 :`G` 0.051269 :`B` 0.051269 :`A` 1.0) :`3` (struct :`R` 0.119538 :`G` 0.088656 :`B` 0.059511 :`A` 1.0) :`4` (struct :`R` 0.000807 :`G` 0.008333 :`A` 1.0) :!type "LinearColor Structure")))