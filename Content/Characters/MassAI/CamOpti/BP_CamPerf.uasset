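; BP_CamPerf is an unfinished performance-capture helper for cameras tagged "CamPerf".
; On BeginPlay it stores the tagged actors in PerfCamd and calls Start, which is currently empty.
; Disconnected nodes would blend the player view to the first camera, record a short trace, toggle FPS, GPU and game stats, and take screenshots between delays, but none of them run.
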(event `self.ReceiveBeginPlay`
  (bind _outactors (`GameplayStatics.GetAllActorsWithTag` "CamPerf"))
  (set `self.PerfCamd` _outactors)
  (`self.Start`))

(event `Start`)

(fn `UserConstructionScript`)