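; Crowd NPC Blueprint that renders a randomizable modular character as Vertex Animation Texture (VAT) meshes through a Niagara system.
; The construction script optionally randomizes indices for skeleton, body, skin, hair and outfit, which getters resolve against CrowdDataAsset into a character definition.
; On BeginPlay it spawns Niagara on Mesh, then pushes part meshes, animation frame range and skin/hair parameters to it.
; Beard and mustache always receive a placeholder box mesh.
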(event `self.ReceiveBeginPlay`
  (bind _returnvalue (`NiagaraFunctionLibrary.SpawnSystemAttached` (`self.NiagaraSystemVAT`) (`self.Mesh`) "None" (0.0 0.0 0.0) (struct) "KeepRelativeOffset" false true "ManualRelease"))
  (set `self.NiagaraParticleVAT` _returnvalue)
  (`self.VATAttribution`))

(fn `GetBodyOutfitDefinition`
  (params (GenderDefinition :type "/Game/CitySampleCrowd/Character/Shared/Structs/CrowdSkeletonDefinition Structure (by ref)") (BodyType :type "/Game/CitySampleCrowd/Character/Shared/Enums/CrowdBodyType Enum" :default "NewEnumerator0"))
  (returns (BodyOutfitDefinition :type "/Game/CitySampleCrowd/Character/Shared/Structs/CrowdBodyOutfitDefinition Structure"))
  (bind (_normalweight _overweight _underweight) (break `/Game/CitySampleCrowd/Character/Shared/Structs/CrowdSkeletonDefinition` GenderDefinition))
  (switch `/Game/CitySampleCrowd/Character/Shared/Enums/CrowdBodyType` BodyType
    (:`NewEnumerator0`
      (return _normalweight))
    (:`NewEnumerator1`
      (return _overweight))
    (:`NewEnumerator2`
      (return _underweight))))

(fn `GetBodyOutiftDefinitionData`
  (params (CrowdBodyOutfitDefinition :type "/Game/CitySampleCrowd/Character/Shared/Structs/CrowdBodyOutfitDefinition Structure (by ref)") (HeadIndex :type Integer) (OutiftIndex :type Integer) (AccessoryIndex :type Integer) (ScaleFactorIndex :type Integer))
  (returns (BodyDefinition :type "/Game/CitySampleCrowd/Character/Shared/Structs/CrowdBodyDefinition Structure") (OutfitDefinition :type "/Game/CitySampleCrowd/Character/Shared/Structs/CrowdOutfitDefinition Structure") (Head :type "SkeletalMesh Soft Object Reference") (HeadVAT :type "/Game/CitySampleCrowd/Character/Shared/Structs/CrowdHeadDefinition Structure") (AccessoryDefinition :type "/Game/CitySampleCrowd/Character/Shared/Structs/CrowdAccessoryDefinition Structure") (ScaleFactor :type "Float (single-precision)") (Animations :type "/Game/CitySampleCrowd/Character/Shared/Structs/CrowdAnimationDefinition Structure"))
  (bind (_body _heads _headsvat _outfits _scalefactors _accessories _animations) (break `/Game/CitySampleCrowd/Character/Shared/Structs/CrowdBodyOutfitDefinition` CrowdBodyOutfitDefinition))
  (return _body (`self.GetSafeCopy` _outfits OutiftIndex) (`self.GetSafeCopy` _heads HeadIndex) (`self.GetSafeCopy` _headsvat HeadIndex) (`self.GetSafeCopy` _accessories AccessoryIndex) (`self.GetSafeCopy` _scalefactors ScaleFactorIndex) _animations))

(fn `GetCharacterDefinition`
  (returns (CharacterDefinition :type "/Game/CitySampleCrowd/Character/Shared/Structs/CrowdCharacterDefinition Structure"))
  (bind _skeletondefinition (`self.GetSkeletonDefinition` (`self.CrowdDataAsset`) (`self.Skeleton`)))
  (bind (_hairdefinition _eyebrowsdefinition _mustachedfinition _bearddefinition) (`self.GetHairDefinitions` _skeletondefinition (`self.HairIndex`) (`self.EyebrowsIndex`) (`self.MustacheIndex`) (`self.BeardIndex`)))
  (bind (_skintexturemodifierdefinition _skintexturedefinition) (`self.GetSkinTextureDefinition` _skeletondefinition (`self.SkinTextureIndex`) (`self.SkinTextureModifierIndex`)))
  (bind (_bodydefinition _outfitdefinition _head _headvat _accessorydefinition _scalefactor _animations) (`self.GetBodyOutiftDefinitionData` (`self.GetBodyOutfitDefinition` _skeletondefinition (`self.Body Shape`)) (`self.HeadIndex`) (`self.OutfitIndex`) (`self.AccessoryIndex`) (`self.ScaleFactorIndex`)))
  (return (make `/Game/CitySampleCrowd/Character/Shared/Structs/CrowdCharacterDefinition` _bodydefinition _head _headvat _outfitdefinition _accessorydefinition (`self.GetHairColorDefinition` (`self.CrowdDataAsset`) (`self.HairColorIndex`)) (`self.GetOutfitMaterialDefinition` _skeletondefinition (`self.Outfit Material Index`)) _skintexturedefinition _skintexturemodifierdefinition _scalefactor (`self.PatternColorIndex`) (`self.PatternOptionIndex`) _hairdefinition _eyebrowsdefinition _mustachedfinition _bearddefinition _animations)))

(fn `GetHairColorDefinition`
  (params (DataAsset :type "/Game/CitySampleCrowd/Blueprints/BP_CrowdCharacterDataAsset Object Reference") (HairColorIndex :type Integer))
  (returns (HairColorDefinition :type "/Game/CitySampleCrowd/Character/Shared/Structs/CrowdHairColorDefinition Structure"))
  (return (`self.GetSafeCopy` (`/Game/CitySampleCrowd/Blueprints/BP_CrowdCharacterDataAsset.HairColors` DataAsset) HairColorIndex)))

(fn `GetHairDefinitions`
  (params (GenderDefinition :type "/Game/CitySampleCrowd/Character/Shared/Structs/CrowdSkeletonDefinition Structure (by ref)") (HairIndex :type Integer) (EyebrowsIndex :type Integer) (MustacheIndex :type Integer) (BeardIndex :type Integer))
  (returns (HairDefinition :type "/Game/CitySampleCrowd/Character/Shared/Structs/CrowdHairDefinition Structure") (EyebrowsDefinition :type "/Game/CitySampleCrowd/Character/Shared/Structs/CrowdHairDefinition Structure") (MustacheDfinition :type "/Game/CitySampleCrowd/Character/Shared/Structs/CrowdHairDefinition Structure") (BeardDefinition :type "/Game/CitySampleCrowd/Character/Shared/Structs/CrowdHairDefinition Structure"))
  (bind ((`HairDefinitions_44_0953ADF4435026AD558912B05090BE99` _hairdefinitions) (`EyebrowsDefinitions_43_D3E07A764729C0980C889487A6FE6B92` _eyebrowsdefinitions) (`MustacheDefinitions_47_D780CE3449C6958165D7DEB5C2CA860D` _mustachedefinitions) (`BeardDefinitions_48_7B35170C47DDECC01EA02AB6A12C9737` _bearddefinitions)) (break `/Game/CitySampleCrowd/Character/Shared/Structs/CrowdSkeletonDefinition` GenderDefinition))
  (return (`self.GetSafeCopy` _hairdefinitions HairIndex) (`self.GetSafeCopy` _eyebrowsdefinitions EyebrowsIndex) (`self.GetSafeCopy` _mustachedefinitions MustacheIndex) (`self.GetSafeCopy` _bearddefinitions BeardIndex)))

(fn `GetOutfitMaterialDefinition`
  (params (GenderDefinition :type "/Game/CitySampleCrowd/Character/Shared/Structs/CrowdSkeletonDefinition Structure (by ref)") (OutfitMaterialIndex :type Integer))
  (returns (OutfitMaterialDefinition :type "/Game/CitySampleCrowd/Character/Shared/Structs/CrowdOutfitMaterialDefinition Structure"))
  (return (`self.GetSafeCopy` (`.OutfitMaterials_53_77BBD6784F5366F598F6019DB6CF60F8` (break `/Game/CitySampleCrowd/Character/Shared/Structs/CrowdSkeletonDefinition` GenderDefinition)) OutfitMaterialIndex)))

(fn `GetSkeletonDefinition`
  (params (DataAsset :type "/Game/CitySampleCrowd/Blueprints/BP_CrowdCharacterDataAsset Object Reference") (Skeleton :type "/Game/CitySampleCrowd/Character/Shared/Enums/CrowdSkeleton Enum" :default "NewEnumerator0"))
  (returns (SkeletonDefinition :type "/Game/CitySampleCrowd/Character/Shared/Structs/CrowdSkeletonDefinition Structure"))
  (switch `/Game/CitySampleCrowd/Character/Shared/Enums/CrowdSkeleton` Skeleton
    (:`NewEnumerator0`
      (return (`/Game/CitySampleCrowd/Blueprints/BP_CrowdCharacterDataAsset.Skeleton A` DataAsset)))
    (:`NewEnumerator1`
      (return (`/Game/CitySampleCrowd/Blueprints/BP_CrowdCharacterDataAsset.Skeleton B` DataAsset)))))

(fn `GetSkinTextureDefinition`
  (params (GenderDefinition :type "/Game/CitySampleCrowd/Character/Shared/Structs/CrowdSkeletonDefinition Structure (by ref)") (SkinTextureIndex :type Integer) (SkinTextureModifierIndex :type Integer))
  (returns (SkinTextureModifierDefinition :type "/Game/CitySampleCrowd/Character/Shared/Structs/CrowdSkinTextureModifierDefinition Structure") (SkinTextureDefinition :type "/Game/CitySampleCrowd/Character/Shared/Structs/CrowdSkinTextureDefinition Structure"))
  (bind (_texture _texturemodifiers) (break `/Game/CitySampleCrowd/Character/Shared/Structs/CrowdSkinMaterialDefinition` (`self.GetSafeCopy` (`.SkinMaterials_15_21D154494E914454F248EDA6BF5BF9FD` (break `/Game/CitySampleCrowd/Character/Shared/Structs/CrowdSkeletonDefinition` GenderDefinition)) SkinTextureIndex)))
  (return (`self.GetSafeCopy` _texturemodifiers SkinTextureModifierIndex) _texture))

(fn `SetRandom`
  (if (not (`self.RandomFace`))
    ;[1 1 1] Gender
    (switch `int` (`KismetMathLibrary.RandomIntegerInRange` 0 1)
      (:`Default`
        (set `self.Skeleton` "NewEnumerator1" :!label _label))
      (:`0`
        (set `self.Skeleton` "NewEnumerator0"))
      (:`1`
        (goto _label))))
  ;[1 1 1] BodyType
  (switch `int` (`KismetMathLibrary.RandomIntegerInRange` 0 2)
    (:`Default`
      (set `self.Body Shape` "NewEnumerator0" :!label _label_2))
    (:`0`
      (set `self.Body Shape` "NewEnumerator1"))
    (:`1`
      (set `self.Body Shape` "NewEnumerator2"))
    (:`2`
      (goto _label_2)))
  ;[1 1 1] Head Index
  (set `self.HeadIndex` (`KismetMathLibrary.RandomIntegerInRange` 0 2))
  ;[1 1 1] SkinTexture
  (set `self.SkinTextureIndex` (`KismetMathLibrary.RandomIntegerInRange` 0 5))
  ;[1 1 1] SkinTextureModifier
  (set `self.SkinTextureModifierIndex` (`KismetMathLibrary.RandomIntegerInRange` 0 35))
  ;[1 1 1] Hair
  (set `self.HairIndex` (`KismetMathLibrary.RandomIntegerInRange` 0 4))
  ;[1 1 1] HairColor
  (set `self.HairColorIndex` (`KismetMathLibrary.RandomIntegerInRange` 0 7))
  ;[1 1 1] Outfit
  (if (not (`self.RandomFace`))
    (set `self.OutfitIndex` (select `int` (`KismetMathLibrary.Conv_ByteToInt` (`self.NPCType`)) :`0` (`KismetMathLibrary.RandomIntegerInRange` 0 3) :`1` (select `int` (`KismetMathLibrary.Conv_ByteToInt` (`self.Skeleton`)) :`0` (select `int` (`KismetMathLibrary.RandomIntegerInRange` 0 1) :`0` 0 :`1` 13) :`1` (select `int` (`KismetMathLibrary.RandomIntegerInRange` 0 2) :`0` 2 :`1` 5 :`2` 15))))
    ;[1 1 1] PatternOption
    (set `self.PatternOptionIndex` (`KismetMathLibrary.RandomIntegerInRange` 0 15))
    ;[1 1 1] PatternColor
    (set `self.PatternColorIndex` (`KismetMathLibrary.RandomIntegerInRange` 0 3)))
  ;[1 1 1] Accessory (setting always to zero for now)
  (set `self.AccessoryIndex` (`KismetMathLibrary.RandomIntegerInRange` 0 11))
  ;[1 1 1] ScaleFactor
  (set `self.ScaleFactorIndex` (`KismetMathLibrary.RandomIntegerInRange` 0 3)))

(fn `UserConstructionScript`
  (if (`self.RandomFace`)
    (`self.SetRandom`))
  ;[1 1 1] Randomize Options
  (if (`self.RandomOptions`)
    (`self.SetRandom`)))

(fn `VATAttribution`
  (bind _niagaraparticlevat (`self.NiagaraParticleVAT`))
  (bind (_bodydefinition _head _headvat _outfitdefinition _accessorydefinition _haircolordefinition _outfitmaterialdefinition _skintexturedefinition _skintexturemodifierdefinition _scalefactor _patterncolorindex _patternoptionindex _hairdefinition _eyebrowsdefinition _mustachedefinition _bearddefinition) (break `/Game/CitySampleCrowd/Character/Shared/Structs/CrowdCharacterDefinition` (`self.GetCharacterDefinition`)))
  (bind (_hairmelanin _hairredness _hairroughness) (break `/Game/CitySampleCrowd/Character/Shared/Structs/CrowdHairColorDefinition` _haircolordefinition))
  (bind (_top _bottom _shoes _vat_top _vat_bottom _vat_shoes) (break `/Game/CitySampleCrowd/Character/Shared/Structs/CrowdOutfitDefinition` _outfitdefinition))
  (bind _dataassetvat (break `/Game/CitySampleCrowd/Character/Shared/Structs/CrowdVATDefinition` _vat_bottom))
  (bind _dataassetvat_2 (break `/Game/CitySampleCrowd/Character/Shared/Structs/CrowdVATDefinition` (`.VAT_52_7B2E92D3444C784036DD33A01DFA67DD` (break `/Game/CitySampleCrowd/Character/Shared/Structs/CrowdHeadDefinition` _headvat))))
  (bind _dataassetvat_3 (break `/Game/CitySampleCrowd/Character/Shared/Structs/CrowdVATDefinition` (`.VAT_30_A8D3743345C745E384DDD89995D830A3` (break `/Game/CitySampleCrowd/Character/Shared/Structs/CrowdHairDefinition` _hairdefinition))))
  (bind _dataassetvat_4 (break `/Game/CitySampleCrowd/Character/Shared/Structs/CrowdVATDefinition` _vat_shoes))
  (bind _dataassetvat_5 (break `/Game/CitySampleCrowd/Character/Shared/Structs/CrowdVATDefinition` (`.VAT_18_BE77C97A448BD4BCCE583A9BFA047B33` (break `/Game/CitySampleCrowd/Character/Shared/Structs/CrowdBodyDefinition` _bodydefinition))))
  (bind _dataassetvat_6 (break `/Game/CitySampleCrowd/Character/Shared/Structs/CrowdVATDefinition` _vat_top))
  (bind (_output_startframe _output_endframe) (break `AnimToTextureAnimInfo` (`|GetArrayItem` (`AnimToTextureDataAsset.Animations` _dataassetvat_6) (`KismetMathLibrary.Conv_ByteToInt` (`self.Anim Index`)))))
  (bind _returnvalue (select `bool` (`KismetSystemLibrary.IsValid` _dataassetvat_2) :`true` (`AnimToTextureDataAsset.BP_GetStaticMesh` _dataassetvat_2)))
  (bind _returnvalue_2 (select `bool` (`KismetSystemLibrary.IsValid` _dataassetvat_3) :`true` (`AnimToTextureDataAsset.BP_GetStaticMesh` _dataassetvat_3)))
  (bind _returnvalue_3 (select `bool` (`KismetSystemLibrary.IsValid` _dataassetvat_4) :`true` (`AnimToTextureDataAsset.BP_GetStaticMesh` _dataassetvat_4)))
  (bind _returnvalue_4 (select `bool` (`KismetSystemLibrary.IsValid` _dataassetvat) :`true` (`AnimToTextureDataAsset.BP_GetStaticMesh` _dataassetvat)))
  (bind _returnvalue_5 (select `bool` (`KismetSystemLibrary.IsValid` _dataassetvat_6) :`true` (`AnimToTextureDataAsset.BP_GetStaticMesh` _dataassetvat_6)))
  (bind _returnvalue_6 (select `bool` (`KismetSystemLibrary.IsValid` _dataassetvat_5) :`true` (`AnimToTextureDataAsset.BP_GetStaticMesh` _dataassetvat_5)))
  ;[1 1 1] FrameOffset
  (`NiagaraComponent.SetVariableFloat` _niagaraparticlevat "Test" (`KismetMathLibrary.Conv_IntToDouble` _output_startframe))
  ;[1 1 1] NumFrame
  (`NiagaraComponent.SetVariableFloat` _niagaraparticlevat "Test2" (`KismetMathLibrary.Conv_IntToDouble` (- _output_endframe _output_startframe)))
  ;[1 1 1] Face & Hair Parameter
  ;;[1 1 1] Atlas Selector
  (`NiagaraComponent.SetVariableFloat` _niagaraparticlevat "AtlasSelector" (`KismetMathLibrary.Conv_IntToDouble` (`.TextureAtlasIndex_2_ABCDAB8D4F5C30DC9AF7DC9C34D5A278` (break `/Game/CitySampleCrowd/Character/Shared/Structs/CrowdSkinTextureDefinition` _skintexturedefinition))))
  ;;[1 1 1] HairMelanin
  (`NiagaraComponent.SetVariableFloat` _niagaraparticlevat "HairMelanin" _hairmelanin)
  ;;[1 1 1] HairRedness
  (`NiagaraComponent.SetVariableFloat` _niagaraparticlevat "HairRedness" _hairredness)
  ;;[1 1 1] HairRoughness
  (`NiagaraComponent.SetVariableFloat` _niagaraparticlevat "HairRoughness" _hairroughness)
  ;[1 1 1] Attribution Modèle VAT
  (if (`KismetSystemLibrary.IsValid` _returnvalue_5)
    ;;[1 1 1] TOP
    (`NiagaraComponent.SetVariableStaticMesh` _niagaraparticlevat "Top" _returnvalue_5))
  (if (`KismetSystemLibrary.IsValid` _returnvalue_6)
    ;;[1 1 1] BODY
    (`NiagaraComponent.SetVariableStaticMesh` _niagaraparticlevat "Body" _returnvalue_6))
  (if (`KismetSystemLibrary.IsValid` _returnvalue_4)
    ;;[1 1 1] Bottom
    (`NiagaraComponent.SetVariableStaticMesh` _niagaraparticlevat "Bottom" _returnvalue_4))
  (if (`KismetSystemLibrary.IsValid` _returnvalue)
    ;;[1 1 1] Face
    (`NiagaraComponent.SetVariableStaticMesh` _niagaraparticlevat "Face" _returnvalue))
  (if (`KismetSystemLibrary.IsValid` _returnvalue_3)
    ;;[1 1 1] Shoes
    (`NiagaraComponent.SetVariableStaticMesh` _niagaraparticlevat "Shoes" _returnvalue_3))
  (if (`KismetSystemLibrary.IsValid` _returnvalue_2)
    ;;[1 1 1] Hair*
    (`NiagaraComponent.SetVariableStaticMesh` _niagaraparticlevat "Hair" _returnvalue_2))
  ;;[1 1 1] Beard
  (`NiagaraComponent.SetVariableStaticMesh` _niagaraparticlevat "Beard" "/Engine/Functions/Engine_MaterialFunctions02/SupportFiles/1x1x1_Box_Pivot_-XYZ.1x1x1_Box_Pivot_-XYZ")
  ;;[1 1 1] Mustache
  (`NiagaraComponent.SetVariableStaticMesh` _niagaraparticlevat "Mustache" "/Engine/Functions/Engine_MaterialFunctions02/SupportFiles/1x1x1_Box_Pivot_-XYZ.1x1x1_Box_Pivot_-XYZ")
  (`FXSystemComponent.SetAutoAttachmentParameters` _niagaraparticlevat null "None" "SnapToTarget" "SnapToTarget" "KeepRelative")
  (set `self.NiagaraSystemVAT` (`NiagaraComponent.GetAsset` _niagaraparticlevat)))