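; Modular crowd NPC whose appearance is assembled in the Construction Script from CrowdDataAsset, using skeleton, body shape and index options that RandomOptions can randomize once.
; The resolved character definition drives meshes following a leader pose, a socketed accessory, grooms and scale.
; Groom bindings are looked up by face and groom asset names.
; Dynamic materials apply skin, hair color, baked groom maps and outfit patterns, which slots can inherit through driven chains.
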(event `self.ReceiveBeginPlay`)

(fn `AttachAccessory`
  (params (AccessoryDefinition :type "/Game/CitySampleCrowd/Character/Shared/Structs/CrowdAccessoryDefinition Structure (by ref)"))
  (bind (_mesh _socketname) (break `/Game/CitySampleCrowd/Character/Shared/Structs/CrowdAccessoryDefinition` AccessoryDefinition))
  (if (`SceneComponent.DoesSocketExist` (`self.SkeletalMesh`) _socketname)
    ;[1 1 1] Set StaticMesh
    (bind _returnvalue (`KismetSystemLibrary.LoadAsset_Blocking` _mesh))
    (bind _asstatic_mesh (cast `StaticMesh` _returnvalue)
      (:`then`
        (`StaticMeshComponent.SetStaticMesh` (`self.Accessory`) _asstatic_mesh)
        ;[1 1 1] Attach Component to Socket
        (`SceneComponent.K2_AttachToComponent` (`self.Accessory`) (`self.SkeletalMesh`) _socketname "KeepRelative" "KeepRelative" "KeepRelative" true))
      (:`CastFailed`
        (`StaticMeshComponent.SetStaticMesh` (`self.Accessory`) null) ; Set Empty
      ))))

(fn `CreateDynamicMaterialInstance`
  (params (MeshComponent :type "MeshComponent Object Reference") (MaterialSlotName :type Name))
  (returns (MaterialInstance :type "MaterialInstanceDynamic Object Reference"))
  (locals (ElementIndex :type Integer :default 0))
  (`|ExecutionSequence`
    (:`then_0`
      (bind _asskeletal_mesh_component (cast `SkeletalMeshComponent` MeshComponent))
      (bind _materialinstance (`self.CreateSkeletalMeshDynamicMaterialInstance` _asskeletal_mesh_component MaterialSlotName))
      (return _materialinstance))
    (:`then_1`
      (bind _asstatic_mesh_component (cast `StaticMeshComponent` MeshComponent))
      (bind _returnvalue (`self.CreateStaticMeshDynamicMaterialInstance` _asstatic_mesh_component MaterialSlotName))
      (return _returnvalue))
    (:`then_2`
      (bind _asgroom_component (cast `GroomComponent` MeshComponent))
      (bind _materialinstance_2 (`self.CreateGroomAssetDynamicMaterialInstance` _asgroom_component MaterialSlotName))
      (return _materialinstance_2))))

(fn `CreateGroomAssetDynamicMaterialInstance`
  (params (GroomComponent :type "GroomComponent Object Reference") (MaterialSlotName :type Name))
  (returns (MaterialInstance :type "MaterialInstanceDynamic Object Reference"))
  (bind _returnvalue (`MeshComponent.GetMaterialIndex` GroomComponent MaterialSlotName))
  (bind _returnvalue_2 (`KismetStringLibrary.Conv_StringToName` (`KismetStringLibrary.Concat_StrStr` (`KismetStringLibrary.Conv_NameToString` MaterialSlotName) "_DynInst")))
  (switch `int` _returnvalue
    (:`0`
      (bind _returnvalue_3 (`PrimitiveComponent.CreateDynamicMaterialInstance` GroomComponent _returnvalue "/Game/CitySampleCrowd/Character/Shared/Materials/MetaHuman/MI_Hair.MI_Hair" _returnvalue_2)) ; Strand
      (return _returnvalue_3))
    (:`1`
      (bind _returnvalue_4 (`PrimitiveComponent.CreateDynamicMaterialInstance` GroomComponent _returnvalue "/Game/CitySampleCrowd/Character/Shared/Materials/MetaHuman/MI_Facial_Hair.MI_Facial_Hair" _returnvalue_2)) ; Cards
      (return _returnvalue_4))
    (:`2`
      (bind _returnvalue_5 (`PrimitiveComponent.CreateDynamicMaterialInstance` GroomComponent _returnvalue "/Game/CitySampleCrowd/Character/Shared/Materials/MetaHuman/MI_Hair_Helmet.MI_Hair_Helmet" _returnvalue_2)) ; Helmets
      (return _returnvalue_5))))

(fn `CreateSkeletalMeshDynamicMaterialInstance`
  (params (SkeletalMeshComponent :type "SkeletalMeshComponent Object Reference") (MaterialSlotName :type Name))
  (returns (MaterialInstance :type "MaterialInstanceDynamic Object Reference"))
  (locals (L_ElementIndex :type Integer :default 0))
  (bind _returnvalue (`SkeletalMeshComponent.GetSkeletalMeshAsset` SkeletalMeshComponent))
  (bind _materials (`SkeletalMesh.Materials` _returnvalue))
  (bind ((`MaterialInterface` _materialinterface) (`MaterialSlotName` _materialslotname)) (break `SkeletalMaterial` (`|GetArrayItem` _materials (`local.L_ElementIndex`))))
  (set `local.L_ElementIndex` (`MeshComponent.GetMaterialIndex` SkeletalMeshComponent MaterialSlotName))
  (`/Engine/EditorBlueprintResources/StandardMacros.IsValid` _returnvalue
    (:`Is Valid`
      (if (`KismetArrayLibrary.Array_IsValidIndex` _materials (`local.L_ElementIndex`))
        (`/Engine/EditorBlueprintResources/StandardMacros.IsValid` _materialinterface
          (:`Is Valid`
            (bind _returnvalue_2 (`PrimitiveComponent.CreateDynamicMaterialInstance` SkeletalMeshComponent (`local.L_ElementIndex`) _materialinterface (`KismetStringLibrary.Conv_StringToName` (`KismetStringLibrary.Concat_StrStr` (`KismetStringLibrary.Conv_NameToString` _materialslotname) "_DynInst"))))
            (return _returnvalue_2)))))
    (:`Is Not Valid`
      (return null))))

(fn `CreateStaticMeshDynamicMaterialInstance`
  (params (StaticMeshComponent :type "StaticMeshComponent Object Reference") (MaterialSlotName :type Name))
  (returns (ReturnValue :type "MaterialInstanceDynamic Object Reference"))
  (bind _staticmesh (`StaticMeshComponent.StaticMesh` StaticMeshComponent))
  (bind _returnvalue (`StaticMesh.GetMaterialIndex` _staticmesh MaterialSlotName))
  (bind _returnvalue_2 (`PrimitiveComponent.CreateDynamicMaterialInstance` StaticMeshComponent _returnvalue (`StaticMesh.GetMaterial` _staticmesh _returnvalue) (`KismetStringLibrary.Conv_StringToName` (`KismetStringLibrary.Concat_StrStr` (`KismetStringLibrary.Conv_NameToString` MaterialSlotName) "_DynInst"))))
  (return _returnvalue_2))

(fn `GetBodyOutfitDefinition`
  (params (GenderDefinition :type "/Game/CitySampleCrowd/Character/Shared/Structs/CrowdSkeletonDefinition Structure (by ref)") (BodyType :type "/Game/CitySampleCrowd/Character/Shared/Enums/CrowdBodyType Enum" :default "NewEnumerator0"))
  (returns (BodyOutfitDefinition :type "/Game/CitySampleCrowd/Character/Shared/Structs/CrowdBodyOutfitDefinition Structure"))
  (bind (_skinmaterials _outfitmaterials _groombindings _hairdefinitions _eyebrowsdefinitions _mustachedefinitions _bearddefinitions _normalweight _overweight _underweight) (break `/Game/CitySampleCrowd/Character/Shared/Structs/CrowdSkeletonDefinition` GenderDefinition))
  (switch `/Game/CitySampleCrowd/Character/Shared/Enums/CrowdBodyType` BodyType
    (:`NewEnumerator0`
      (return _normalweight))
    (:`NewEnumerator1`
      (return _overweight))
    (:`NewEnumerator2`
      (return _underweight))))

(fn `GetBodyOutiftDefinitionData`
  (params (CrowdBodyOutfitDefinition :type "/Game/CitySampleCrowd/Character/Shared/Structs/CrowdBodyOutfitDefinition Structure (by ref)") (HeadIndex :type Integer) (OutiftIndex :type Integer) (AccessoryIndex :type Integer) (ScaleFactorIndex :type Integer))
  (returns (BodyDefinition :type "/Game/CitySampleCrowd/Character/Shared/Structs/CrowdBodyDefinition Structure") (OutfitDefinition :type "/Game/CitySampleCrowd/Character/Shared/Structs/CrowdOutfitDefinition Structure") (Head :type "SkeletalMesh Soft Object Reference") (AccessoryDefinition :type "/Game/CitySampleCrowd/Character/Shared/Structs/CrowdAccessoryDefinition Structure") (ScaleFactor :type "Float (single-precision)"))
  (bind (_body _heads _outfits _scalefactors _accessories) (break `/Game/CitySampleCrowd/Character/Shared/Structs/CrowdBodyOutfitDefinition` CrowdBodyOutfitDefinition))
  (return _body (`self.GetSafeCopy` _outfits OutiftIndex) (`self.GetSafeCopy` _heads HeadIndex) (`self.GetSafeCopy` _accessories AccessoryIndex) (`self.GetSafeCopy` _scalefactors ScaleFactorIndex)))

(fn `GetBodyType`
  (returns (BodyType :type "/Game/CitySampleCrowd/Character/Shared/Enums/CrowdBodyType Enum"))
  (return (`self.Body Shape`)))

(fn `GetCharacterDefinition`
  (returns (CharacterDefinition :type "/Game/CitySampleCrowd/Character/Shared/Structs/CrowdCharacterDefinition Structure"))
  (bind _skeletondefinition (`self.GetSkeletonDefinition` (`self.CrowdDataAsset`) (`self.Skeleton`)))
  (bind (_hairdefinition _eyebrowsdefinition _mustachedfinition _bearddefinition) (`self.GetHairDefinitions` (`self.HairIndex`) (`self.EyebrowsIndex`) (`self.MustacheIndex`) (`self.BeardIndex`) _skeletondefinition))
  (bind (_skintexturemodifierdefinition _skintexturedefinition) (`self.GetSkinTextureDefinition` (`self.SkinTextureIndex`) (`self.SkinTextureModifierIndex`) _skeletondefinition))
  (bind (_bodydefinition _outfitdefinition _head _accessorydefinition _scalefactor) (`self.GetBodyOutiftDefinitionData` (`self.HeadIndex`) (`self.OutfitIndex`) (`self.AccessoryIndex`) (`self.ScaleFactorIndex`) (`self.GetBodyOutfitDefinition` (`self.Body Shape`) _skeletondefinition)))
  (return (make `/Game/CitySampleCrowd/Character/Shared/Structs/CrowdCharacterDefinition` _bodydefinition _head _outfitdefinition _accessorydefinition (`self.GetHairColorDefinition` (`self.CrowdDataAsset`) (`self.HairColorIndex`)) (`self.GetOutfitMaterialDefinition` (`self.OutfitMaterialIndex`) _skeletondefinition) _skintexturedefinition _skintexturemodifierdefinition _scalefactor (`self.PatternColorIndex`) (`self.PatternOptionIndex`) _hairdefinition _eyebrowsdefinition _mustachedfinition _bearddefinition)))

(fn `GetHairColorDefinition`
  (params (DataAsset :type "/Game/CitySampleCrowd/Blueprints/BP_CrowdCharacterDataAsset Object Reference") (HairColorIndex :type Integer))
  (returns (HairColorDefinition :type "/Game/CitySampleCrowd/Character/Shared/Structs/CrowdHairColorDefinition Structure"))
  (return (`self.GetSafeCopy` (`/Game/CitySampleCrowd/Blueprints/BP_CrowdCharacterDataAsset.HairColors` DataAsset) HairColorIndex)))

(fn `GetHairDefinitions`
  (params (GenderDefinition :type "/Game/CitySampleCrowd/Character/Shared/Structs/CrowdSkeletonDefinition Structure (by ref)") (HairIndex :type Integer) (EyebrowsIndex :type Integer) (MustacheIndex :type Integer) (BeardIndex :type Integer))
  (returns (HairDefinition :type "/Game/CitySampleCrowd/Character/Shared/Structs/CrowdHairDefinition Structure") (EyebrowsDefinition :type "/Game/CitySampleCrowd/Character/Shared/Structs/CrowdHairDefinition Structure") (MustacheDfinition :type "/Game/CitySampleCrowd/Character/Shared/Structs/CrowdHairDefinition Structure") (BeardDefinition :type "/Game/CitySampleCrowd/Character/Shared/Structs/CrowdHairDefinition Structure"))
  (bind ((`HairDefinitions_44_0953ADF4435026AD558912B05090BE99` _hairdefinitions) (`EyebrowsDefinitions_43_D3E07A764729C0980C889487A6FE6B92` _eyebrowsdefinitions) (`MustacheDefinitions_47_D780CE3449C6958165D7DEB5C2CA860D` _mustachedefinitions) (`BeardDefinitions_48_7B35170C47DDECC01EA02AB6A12C9737` _bearddefinitions)) (break `/Game/CitySampleCrowd/Character/Shared/Structs/CrowdSkeletonDefinition` GenderDefinition))
  (return (`self.GetSafeCopy` _hairdefinitions HairIndex) (`self.GetSafeCopy` _eyebrowsdefinitions EyebrowsIndex) (`self.GetSafeCopy` _mustachedefinitions MustacheIndex) (`self.GetSafeCopy` _bearddefinitions BeardIndex)))

(fn `GetOutfitMaterialDefinition`
  (params (GenderDefinition :type "/Game/CitySampleCrowd/Character/Shared/Structs/CrowdSkeletonDefinition Structure (by ref)") (OutfitMaterialIndex :type Integer))
  (returns (OutfitMaterialDefinition :type "/Game/CitySampleCrowd/Character/Shared/Structs/CrowdOutfitMaterialDefinition Structure"))
  (return (`self.GetSafeCopy` (`.OutfitMaterials_53_77BBD6784F5366F598F6019DB6CF60F8` (break `/Game/CitySampleCrowd/Character/Shared/Structs/CrowdSkeletonDefinition` GenderDefinition)) OutfitMaterialIndex)))

(fn `GetPatternInfoForSlot`
  (params (MaterialOverrides :type "Map of Name to /Game/CitySampleCrowd/Character/Shared/Structs/CrowdMaterialOverride Structure") (SlotName :type Name) (PatternColorIndex :type Integer) (PatternSelectionIndex :type Integer))
  (returns (PatternColor :type "Color Structure") (PatternInfo :type "/Game/CitySampleCrowd/Character/Shared/Structs/CrowdPatternInfo Structure") (bFound :type Boolean))
  (locals (L_DrivenScaleMultiplier :type "Float (double-precision)" :default 1.0) (L_MaterialOverride :type "/Game/CitySampleCrowd/Character/Shared/Structs/CrowdMaterialOverride Structure") (L_Condition :type Boolean :default true) (L_PatternColor :type "Color Structure") (L_PatternInfo :type "/Game/CitySampleCrowd/Character/Shared/Structs/CrowdPatternInfo Structure"))
  (bind ((`PatternUsage_21_0BFA6A1E41063A6D3CBBC3B8C651A091` _patternusage) (`ComplimentaryColors_17_302B872644700667271B088EADC01A47` _complimentarycolors) (`Patterns_16_7C5408BA4B033275AA2F99BA6586F623` _patterns)) (break `/Game/CitySampleCrowd/Character/Shared/Structs/CrowdMaterialOverride` (`local.L_MaterialOverride`)))
  (bind (_value _returnvalue) (`BlueprintMapLibrary.Map_Find` MaterialOverrides (`.SourceSlot_18_3E7A9CD84A7DEA1E4FEED2AC3CC3C118` (break `/Game/CitySampleCrowd/Character/Shared/Structs/CrowdMaterialOverride` (`local.L_MaterialOverride`)))))
  (set `local.L_MaterialOverride` (`BlueprintMapLibrary.Map_Find` MaterialOverrides SlotName))
  (while (`local.L_Condition`)
    (switch `/Game/CitySampleCrowd/Character/Shared/Enums/CrowdPatternUsage` _patternusage
      (:`NewEnumerator0`
        ;[1 1 1] No Pattern
        (set `local.L_Condition` false))
      (:`NewEnumerator1`
        ;[1 1 1] PatternList
        (if (and (`KismetArrayLibrary.Array_IsNotEmpty` _complimentarycolors) (`KismetArrayLibrary.Array_IsNotEmpty` _patterns))
          (set `local.L_PatternColor` (`self.GetSafeCopy` _complimentarycolors PatternColorIndex))
          (bind _output_get (set `local.L_PatternInfo` (`self.GetSafeCopy` _patterns PatternSelectionIndex)))
          (setmembers `/Game/CitySampleCrowd/Character/Shared/Structs/CrowdPatternInfo` :`StructRef` _output_get :`Scale` (* (`.Scale_5_ABCDAB8D4F5C30DC9AF7DC9C34D5A278` (break `/Game/CitySampleCrowd/Character/Shared/Structs/CrowdPatternInfo` _output_get)) (`local.L_DrivenScaleMultiplier`)))
          (return (`local.L_PatternColor`) (`local.L_PatternInfo`) true)
          (else
            (set `local.L_Condition` false))))
      (:`NewEnumerator2`
        ;[1 1 1] Driven
        (if _returnvalue
          ;;[1 1 1] Update the scale multiplier and then set the current material override to evaluate
          (set `local.L_DrivenScaleMultiplier` (* (`.ScaleMultiplier_19_946AFC864F92A63F07B3A9A02A2AC8A3` (break `/Game/CitySampleCrowd/Character/Shared/Structs/CrowdMaterialOverride` (`local.L_MaterialOverride`))) (`local.L_DrivenScaleMultiplier`)))
          (set `local.L_MaterialOverride` _value)
          (else
            (set `local.L_Condition` false))))))
  (return (`local.L_PatternColor`) (`local.L_PatternInfo`) false))

(fn `GetSkeletonDefinition`
  (params (DataAsset :type "/Game/CitySampleCrowd/Blueprints/BP_CrowdCharacterDataAsset Object Reference") (Skeleton :type "/Game/CitySampleCrowd/Character/Shared/Enums/CrowdSkeleton Enum" :default "NewEnumerator0"))
  (returns (SkeletonDefinition :type "/Game/CitySampleCrowd/Character/Shared/Structs/CrowdSkeletonDefinition Structure"))
  (switch `/Game/CitySampleCrowd/Character/Shared/Enums/CrowdSkeleton` Skeleton
    (:`NewEnumerator0`
      (return (`/Game/CitySampleCrowd/Blueprints/BP_CrowdCharacterDataAsset.Skeleton A` DataAsset)))
    (:`NewEnumerator1`
      (return (`/Game/CitySampleCrowd/Blueprints/BP_CrowdCharacterDataAsset.Skeleton B` DataAsset)))))

(fn `GetSkinTextureDefinition`
  (params (GenderDefinition :type "/Game/CitySampleCrowd/Character/Shared/Structs/CrowdSkeletonDefinition Structure (by ref)") (SkinTextureIndex :type Integer) (SkinTextureModifierIndex :type Integer))
  (returns (SkinTextureModifierDefinition :type "/Game/CitySampleCrowd/Character/Shared/Structs/CrowdSkinTextureModifierDefinition Structure") (SkinTextureDefinition :type "/Game/CitySampleCrowd/Character/Shared/Structs/CrowdSkinTextureDefinition Structure"))
  (bind (_texture _texturemodifiers) (break `/Game/CitySampleCrowd/Character/Shared/Structs/CrowdSkinMaterialDefinition` (`self.GetSafeCopy` (`.SkinMaterials_15_21D154494E914454F248EDA6BF5BF9FD` (break `/Game/CitySampleCrowd/Character/Shared/Structs/CrowdSkeletonDefinition` GenderDefinition)) SkinTextureIndex)))
  (return (`self.GetSafeCopy` _texturemodifiers SkinTextureModifierIndex) _texture))

(fn `SetBakedGroomMap`
  (params (MaterialInstance :type "MaterialInstanceDynamic Object Reference") (AttributeMapName :type Name) (Groom :type "GroomAsset Soft Object Reference") (BakedGroomMap :type "Texture2D Soft Object Reference") (BakedGroomMinimumLOD :type Integer) (LODIndex :type Integer))
  (if (and (or (>= LODIndex BakedGroomMinimumLOD) (!= (`KismetSystemLibrary.IsValidSoftObjectReference` Groom) false)) (`KismetSystemLibrary.IsValidSoftObjectReference` BakedGroomMap))
    (bind _returnvalue (`KismetSystemLibrary.LoadAsset_Blocking` BakedGroomMap))
    (bind _astexture_2d (cast `Texture2D` _returnvalue))
    (`/Engine/EditorBlueprintResources/StandardMacros.IsValid` _astexture_2d
      (:`Is Valid`
        (`MaterialInstanceDynamic.SetTextureParameterValue` MaterialInstance AttributeMapName _astexture_2d)))
    (else
      (`MaterialInstanceDynamic.SetTextureParameterValue` MaterialInstance AttributeMapName "/Game/CitySampleCrowd/Character/Shared/Textures/1x1_BakedGroomTextureBase_VT.1x1_BakedGroomTextureBase_VT") ; Set default texture
    )))

(fn `SetBodyMaterials`
  (params (SkinTextureDefinition :type "/Game/CitySampleCrowd/Character/Shared/Structs/CrowdSkinTextureDefinition Structure") (SkinTextureModifierDefinition :type "/Game/CitySampleCrowd/Character/Shared/Structs/CrowdSkinTextureModifierDefinition Structure"))
  (bind (_textureatlasindex _sourceu _sourcev _albedomultiplier) (break `/Game/CitySampleCrowd/Character/Shared/Structs/CrowdSkinTextureDefinition` SkinTextureDefinition))
  (bind (_offsetu _offsetv) (break `/Game/CitySampleCrowd/Character/Shared/Structs/CrowdSkinTextureModifierDefinition` SkinTextureModifierDefinition))
  (bind _bottom (`self.Bottom`))
  (bind _returnvalue (`MeshComponent.GetMaterialIndex` _bottom "M_Body"))
  (bind _materialinstance (`self.CreateDynamicMaterialInstance` (`self.Body`) "lambert1"))
  (`MaterialInstanceDynamic.SetScalarParameterValue` _materialinstance "AtlasSelector" (`KismetMathLibrary.Conv_IntToDouble` _textureatlasindex))
  (`MaterialInstanceDynamic.SetScalarParameterValue` _materialinstance "MelaninRandomSeed" _offsetu)
  (`MaterialInstanceDynamic.SetScalarParameterValue` _materialinstance "RednessRandomSeed" _offsetv)
  (`MaterialInstanceDynamic.SetScalarParameterValue` _materialinstance "SourceU" _sourceu)
  (`MaterialInstanceDynamic.SetScalarParameterValue` _materialinstance "SourceV" _sourcev)
  (`MaterialInstanceDynamic.SetScalarParameterValue` _materialinstance "AlbedoDataMult" _albedomultiplier)
  ;[1 1 1] Some outfits have exposed skin on the bottom half, if this is the case then we'll have it share the skin material from the upper body to prevent a mismatch
  (`/Engine/EditorBlueprintResources/StandardMacros.IsValid` _bottom
    (:`Is Valid`
      (if (>= _returnvalue 0)
        (`PrimitiveComponent.SetMaterial` (`self.Bottom`) _returnvalue _materialinstance)))))

(fn `SetCharacterDefinition`
  (params (CharacterDefinition :type "/Game/CitySampleCrowd/Character/Shared/Structs/CrowdCharacterDefinition Structure"))
  (bind (_bodydefinition _head _outfitdefinition _accessorydefinition _haircolordefinition _outfitmaterialdefinition _skintexturedefinition _skintexturemodifierdefinition _scalefactor _patterncolorindex _patternoptionindex _hairdefinition _eyebrowsdefinition _mustachedefinition _bearddefinition) (break `/Game/CitySampleCrowd/Character/Shared/Structs/CrowdCharacterDefinition` CharacterDefinition))
  (bind (_base _body) (break `/Game/CitySampleCrowd/Character/Shared/Structs/CrowdBodyDefinition` _bodydefinition))
  (bind (_top _bottom _shoes) (break `/Game/CitySampleCrowd/Character/Shared/Structs/CrowdOutfitDefinition` _outfitdefinition))
  ;[1 1 1] Meshes
  (`self.SetSkeletalMeshes` _base _body _head _top _bottom _shoes)
  (`self.AttachAccessory` _accessorydefinition)
  ;[1 1 1] Grooms
  (`self.SetGrooms` _hairdefinition _mustachedefinition _bearddefinition)
  (`self.SetGroomBinding`) ; Sets GroomBinding from Lookup
  ;[1 1 1] Materials
  (`self.SetFaceMaterials` _skintexturedefinition _skintexturemodifierdefinition _haircolordefinition _hairdefinition _eyebrowsdefinition _mustachedefinition _bearddefinition)
  (`self.SetGroomsMaterials` _haircolordefinition)
  (`self.SetOutfitMaterials` _patterncolorindex _patternoptionindex _outfitmaterialdefinition)
  (`self.SetBodyMaterials` _skintexturedefinition _skintexturemodifierdefinition)
  ;[1 1 1] Set Scale Factor
  (`SceneComponent.SetRelativeScale3D` (`self.SkeletalMesh`) (`KismetMathLibrary.Conv_DoubleToVector` _scalefactor)))

(fn `SetFaceMaterial`
  (params (MaterialInstance :type "MaterialInstanceDynamic Object Reference") (SkinTextureDefinition :type "/Game/CitySampleCrowd/Character/Shared/Structs/CrowdSkinTextureDefinition Structure (by ref)") (SkinTextureModifierDefinition :type "/Game/CitySampleCrowd/Character/Shared/Structs/CrowdSkinTextureModifierDefinition Structure (by ref)"))
  (locals (L_MaterialInstance :type "MaterialInstanceDynamic Object Reference"))
  (bind (_textureatlasindex _sourceu _sourcev _albedomultiplier) (break `/Game/CitySampleCrowd/Character/Shared/Structs/CrowdSkinTextureDefinition` SkinTextureDefinition))
  (bind (_offsetu _offsetv) (break `/Game/CitySampleCrowd/Character/Shared/Structs/CrowdSkinTextureModifierDefinition` SkinTextureModifierDefinition))
  (`/Engine/EditorBlueprintResources/StandardMacros.IsValid` MaterialInstance
    (:`Is Valid`
      (set `local.L_MaterialInstance` MaterialInstance)
      (`|ExecutionSequence`
        (:`then_0`
          (`MaterialInstanceDynamic.SetScalarParameterValue` (`local.L_MaterialInstance`) "AtlasSelector" (`KismetMathLibrary.Conv_IntToDouble` _textureatlasindex)))
        (:`then_1`
          (`MaterialInstanceDynamic.SetScalarParameterValue` (`local.L_MaterialInstance`) "MelaninRandomSeed" _offsetu))
        (:`then_2`
          (`MaterialInstanceDynamic.SetScalarParameterValue` (`local.L_MaterialInstance`) "RednessRandomSeed" _offsetv))
        (:`then_3`
          (`MaterialInstanceDynamic.SetScalarParameterValue` (`local.L_MaterialInstance`) "SourceU" _sourceu))
        (:`then_4`
          (`MaterialInstanceDynamic.SetScalarParameterValue` (`local.L_MaterialInstance`) "SourceV" _sourcev))
        (:`then_5`
          (`MaterialInstanceDynamic.SetScalarParameterValue` (`local.L_MaterialInstance`) "AlbedoDataMult" _albedomultiplier))))))

(fn `SetFaceMaterials`
  (params (SkinTextureDefinition :type "/Game/CitySampleCrowd/Character/Shared/Structs/CrowdSkinTextureDefinition Structure") (SkinTextureModifierDefinition :type "/Game/CitySampleCrowd/Character/Shared/Structs/CrowdSkinTextureModifierDefinition Structure") (HairColorDefinition :type "/Game/CitySampleCrowd/Character/Shared/Structs/CrowdHairColorDefinition Structure") (HairDefinition :type "/Game/CitySampleCrowd/Character/Shared/Structs/CrowdHairDefinition Structure") (EyebrowsDefinition :type "/Game/CitySampleCrowd/Character/Shared/Structs/CrowdHairDefinition Structure") (MustacheDefinition :type "/Game/CitySampleCrowd/Character/Shared/Structs/CrowdHairDefinition Structure") (BeardDefinition :type "/Game/CitySampleCrowd/Character/Shared/Structs/CrowdHairDefinition Structure"))
  (locals (MaterialInstance :type "MaterialInstanceDynamic Object Reference"))
  (for (_array_element _array_index) (`|MakeArray` "head_shader_shader" "head_LOD1_shader_shader" "head_LOD2_shader_shader" "head_LOD3_shader_shader" "head_LOD4_shader_shader" "head_LOD57_shader_shader" :!type "Name")
    (bind _materialinstance (`self.CreateDynamicMaterialInstance` (`self.Face`) _array_element))
    (`self.SetFaceMaterial` _materialinstance SkinTextureDefinition SkinTextureModifierDefinition) ; Face
    (`self.SetScalpMaterial` _materialinstance HairColorDefinition BeardDefinition "BeardAttributeMap" "FollicleMaskBeard" "BeardMelanin" "BeardRedness" _array_index) ; Beard
    (`self.SetScalpMaterial` _materialinstance HairColorDefinition EyebrowsDefinition "EyebrowsAttributeMap" "None" "EyebrowsMelanin" "EyebrowsRedness" _array_index) ; Eyebrows
    (`self.SetScalpMaterial` _materialinstance HairColorDefinition HairDefinition "HairAttributeMap" "FollicleMaskHair" "HairMelanin" "HairRedness" _array_index) ; Hair
    (`self.SetScalpMaterial` _materialinstance HairColorDefinition MustacheDefinition "MustacheAttributeMap" "FollicleMaskMustache" "MustacheMelanin" "MustacheRedness" _array_index) ; Mustache
  ))

(fn `SetFollicleMask`
  (params (MaterialInstance :type "MaterialInstanceDynamic Object Reference") (FollicleMaskName :type Name) (FollicleMask :type "Object Soft Object Reference (by ref)"))
  (if (!= FollicleMaskName "None")
    (if (`KismetSystemLibrary.IsValidSoftObjectReference` FollicleMask)
      (bind _returnvalue (`KismetSystemLibrary.LoadAsset_Blocking` FollicleMask))
      (bind _astexture_2d (cast `Texture2D` _returnvalue))
      (`MaterialInstanceDynamic.SetTextureParameterValue` MaterialInstance FollicleMaskName _astexture_2d)
      (else
        (`MaterialInstanceDynamic.SetTextureParameterValue` MaterialInstance FollicleMaskName "/Game/CitySampleCrowd/Character/Shared/Textures/Default/T_DefaultMaskTexture_VT.T_DefaultMaskTexture_VT")))))

(fn `SetGroom`
  (params (GroomComponent :type "GroomComponent Object Reference") (HairDefinition :type "/Game/CitySampleCrowd/Character/Shared/Structs/CrowdHairDefinition Structure (by ref)"))
  (bind _returnvalue (`KismetSystemLibrary.LoadAsset_Blocking` (`.Groom_2_ABCDAB8D4F5C30DC9AF7DC9C34D5A278` (break `/Game/CitySampleCrowd/Character/Shared/Structs/CrowdHairDefinition` HairDefinition))))
  (bind _asgroom_asset (cast `GroomAsset` _returnvalue)
    (:`then`
      (`GroomComponent.SetGroomAsset` GroomComponent _asgroom_asset))
    (:`CastFailed`
      (`GroomComponent.SetGroomAsset` GroomComponent null) ; Set Empty
    )))

(fn `SetGroomBinding`
  (locals (L_GroomBindings :type "Map of Name to GroomBindingAsset Object Reference"))
  (bind _returnvalue (`SkeletalMeshComponent.GetSkeletalMeshAsset` (`self.Face`)))
  (bind (_returnvalue_packagename _returnvalue_packagepath _returnvalue_assetname) (break `AssetData` (`AssetRegistryHelpers.CreateAssetData` _returnvalue)))
  (`BlueprintMapLibrary.Map_Clear` (`local.L_GroomBindings`))
  ;[1 1 1] Get All GroomBindings
  (`|ExecutionSequence`
    (:`then_0`
      (for _array_element (`.GroomBindings_23_C06ED3324462B1C9476B4582F2D809A3` (break `/Game/CitySampleCrowd/Character/Shared/Structs/CrowdSkeletonDefinition` (`self.GetSkeletonDefinition` (`self.CrowdDataAsset`) (`self.Skeleton`))))
        (bind _returnvalue_2 (`KismetSystemLibrary.LoadAsset_Blocking` _array_element))
        (bind _asgroom_binding_asset (cast `GroomBindingAsset` _returnvalue_2))
        (bind (_returnvalue_packagename_2 _returnvalue_packagepath_2 _returnvalue_assetname_2) (break `AssetData` (`AssetRegistryHelpers.CreateAssetData` _asgroom_binding_asset)))
        (`BlueprintMapLibrary.Map_Add` (`local.L_GroomBindings`) _returnvalue_assetname_2 _asgroom_binding_asset)))
    (:`then_1`
      (`/Engine/EditorBlueprintResources/StandardMacros.IsValid` _returnvalue
        (:`Is Valid`
          (for _array_element_2 (`|MakeArray` (`self.Mustache2`) (`self.Hair2`) (`self.Beard2`))
            (bind _groomasset (`GroomComponent.GroomAsset` _array_element_2))
            (`/Engine/EditorBlueprintResources/StandardMacros.IsValid` _groomasset
              (:`Is Valid`
                (bind (_returnvalue_packagename_3 _returnvalue_packagepath_3 _returnvalue_assetname_3) (break `AssetData` (`AssetRegistryHelpers.CreateAssetData` _groomasset)))
                (bind _returnvalue_3 (`KismetStringLibrary.Concat_StrStr` "GB_" (`KismetStringLibrary.Conv_NameToString` _returnvalue_assetname) "_" (`KismetStringLibrary.Conv_NameToString` _returnvalue_assetname_3)))
                (bind (_value _returnvalue_4) (`BlueprintMapLibrary.Map_Find` (`local.L_GroomBindings`) (`KismetStringLibrary.Conv_StringToName` _returnvalue_3)))
                (if _returnvalue_4
                  (`GroomComponent.SetBindingAsset` _array_element_2 _value)
                  (else
                    (`KismetSystemLibrary.PrintString` (`KismetStringLibrary.Concat_StrStr` "GroomBinding not found: " _returnvalue_3)))))
              (:`Is Not Valid`
                (`GroomComponent.SetBindingAsset` _array_element_2 null) ; Set Empty
              ))))))))

(fn `SetGrooms`
  (params (HairDefinition :type "/Game/CitySampleCrowd/Character/Shared/Structs/CrowdHairDefinition Structure (by ref)") (MustacheDefinition :type "/Game/CitySampleCrowd/Character/Shared/Structs/CrowdHairDefinition Structure (by ref)") (BeardDefinition :type "/Game/CitySampleCrowd/Character/Shared/Structs/CrowdHairDefinition Structure (by ref)"))
  (`self.SetGroom` (`self.Hair2`) HairDefinition)
  (`self.SetGroom` (`self.Mustache2`) MustacheDefinition)
  (`self.SetGroom` (`self.Beard2`) BeardDefinition))

(fn `SetGroomsMaterials`
  (params (HairColorDefiniion :type "/Game/CitySampleCrowd/Character/Shared/Structs/CrowdHairColorDefinition Structure"))
  (for _array_element (`|MakeArray` (`self.Mustache2`) (`self.Hair2`) (`self.Beard2`))
    (`self.SetHairMaterials` _array_element HairColorDefiniion "hairMelanin" "hairRedness" "HairRoughness")))

(fn `SetHairMaterials`
  (params (HairComponent :type "GroomComponent Object Reference") (HairColorDefiniion :type "/Game/CitySampleCrowd/Character/Shared/Structs/CrowdHairColorDefinition Structure") (MelaninParameterName :type Name) (RednessParameterName :type Name) (RoughnessParameterName :type Name))
  (bind (_hairmelanin _hairredness _hairroughness) (break `/Game/CitySampleCrowd/Character/Shared/Structs/CrowdHairColorDefinition` HairColorDefiniion))
  (for _array_element (`MeshComponent.GetMaterialSlotNames` HairComponent)
    (bind _materialinstance (`self.CreateDynamicMaterialInstance` HairComponent _array_element))
    (`/Engine/EditorBlueprintResources/StandardMacros.IsValid` _materialinstance
      (:`Is Valid`
        (`MaterialInstanceDynamic.SetScalarParameterValue` _materialinstance MelaninParameterName _hairmelanin)
        (`MaterialInstanceDynamic.SetScalarParameterValue` _materialinstance RednessParameterName _hairredness)
        (`MaterialInstanceDynamic.SetScalarParameterValue` _materialinstance RoughnessParameterName _hairroughness)))))

(fn `SetMelaninAndRedless`
  (params (MaterialInstance :type "MaterialInstanceDynamic Object Reference") (MelaninParameterName :type Name) (RednessParameterName :type Name) (CrowdHairColorDefinition :type "/Game/CitySampleCrowd/Character/Shared/Structs/CrowdHairColorDefinition Structure (by ref)"))
  (bind ((`HairMelanin_2_ABCDAB8D4F5C30DC9AF7DC9C34D5A278` _hairmelanin) (`HairRedness_4_EA4B489340889D37F2F5529C76BBC721` _hairredness)) (break `/Game/CitySampleCrowd/Character/Shared/Structs/CrowdHairColorDefinition` CrowdHairColorDefinition))
  ;[1 1 1] Ensure Melanin and Redness matches hair color
  (`MaterialInstanceDynamic.SetScalarParameterValue` MaterialInstance MelaninParameterName _hairmelanin)
  (`MaterialInstanceDynamic.SetScalarParameterValue` MaterialInstance RednessParameterName _hairredness))

(fn `SetOutfitMaterial`
  (params (MeshComponent :type "MeshComponent Object Reference") (PatternColorIndex :type Integer) (PatternOptionIndex :type Integer) (MaterialOverrides :type "Map of Name to /Game/CitySampleCrowd/Character/Shared/Structs/CrowdMaterialOverride Structure"))
  (for _array_element (`MeshComponent.GetMaterialSlotNames` MeshComponent)
    (bind _materialinstance (`self.CreateDynamicMaterialInstance` MeshComponent _array_element))
    (bind (_value _returnvalue) (`BlueprintMapLibrary.Map_Find` MaterialOverrides _array_element))
    (if (and (`KismetSystemLibrary.IsValid` _materialinstance) _returnvalue)
      ;[1 1 1] Apply Parameter Overrides
      (`self.SetOutfitParameterOverrides` (`.ParameterOverrides_3_ABCDAB8D4F5C30DC9AF7DC9C34D5A278` (break `/Game/CitySampleCrowd/Character/Shared/Structs/CrowdMaterialOverride` _value)) _materialinstance)
      ;[1 1 1] Apply Patterns
      (bind (_patterncolor _patterninfo _bfound) (`self.GetPatternInfoForSlot` MaterialOverrides _array_element PatternColorIndex PatternOptionIndex))
      (if _bfound
        (`MaterialInstanceDynamic.SetVectorParameterValue` _materialinstance "A_CrowdColor_pattern" (`self.ReinterpretAsLinear` _patterncolor))
        (bind (_scale _selection _roughnessmultiplier) (break `/Game/CitySampleCrowd/Character/Shared/Structs/CrowdPatternInfo` _patterninfo))
        (`MaterialInstanceDynamic.SetScalarParameterValue` _materialinstance "A_Pattern_Scale" _scale)
        (`MaterialInstanceDynamic.SetScalarParameterValue` _materialinstance "A_Pattern_Select" (`KismetMathLibrary.Conv_IntToDouble` _selection))
        (`MaterialInstanceDynamic.SetScalarParameterValue` _materialinstance "A_Pattern_RoughMult" _roughnessmultiplier)))))

(fn `SetOutfitMaterials`
  (params (PatternColorIndex :type Integer) (PatternOptionIndex :type Integer) (OutfitMaterialDefinition :type "/Game/CitySampleCrowd/Character/Shared/Structs/CrowdOutfitMaterialDefinition Structure (by ref)"))
  (bind _materialoverrides (break `/Game/CitySampleCrowd/Character/Shared/Structs/CrowdOutfitMaterialDefinition` OutfitMaterialDefinition))
  (`|ExecutionSequence`
    (:`then_0`
      ;[1 1 1] Outfit
      (for _array_element (`|MakeArray` (`self.Top`) (`self.Bottom`) (`self.Shoes`))
        (`self.SetOutfitMaterial` _array_element PatternColorIndex PatternOptionIndex _materialoverrides)))
    (:`then_1`
      ;[1 1 1] Accessory
      (`self.SetOutfitMaterial` (`self.Accessory`) PatternColorIndex PatternOptionIndex _materialoverrides))))

(fn `SetOutfitParameterOverrides`
  (params (ParameterOverrides :type "Array of /Game/CitySampleCrowd/Character/Shared/Structs/CrowdMaterialColorOverride Structure") (MaterialInstance :type "MaterialInstanceDynamic Object Reference"))
  (for _array_element ParameterOverrides
    (bind (_parametername _color) (break `/Game/CitySampleCrowd/Character/Shared/Structs/CrowdMaterialColorOverride` _array_element))
    (`MaterialInstanceDynamic.SetVectorParameterValue` MaterialInstance _parametername (`self.ReinterpretAsLinear` _color))))

(fn `SetRandomOptions`
  ;[1 1 1] Gender
  (switch `int` (`KismetMathLibrary.RandomIntegerInRange` 0 1)
    (:`Default`
      (set `self.Skeleton` "NewEnumerator1" :!label _label))
    (:`0`
      (set `self.Skeleton` "NewEnumerator0"))
    (:`1`
      (goto _label)))
  ;[1 1 1] BodyType
  (switch `int` (`KismetMathLibrary.RandomIntegerInRange` 0 2)
    (:`Default`
      (set `self.Body Shape` "NewEnumerator0" :!label _label_2))
    (:`0`
      (set `self.Body Shape` "NewEnumerator1"))
    (:`1`
      (set `self.Body Shape` "NewEnumerator2"))
    (:`2`
      (goto _label_2)))
  ;[1 1 1] Head Index
  (set `self.HeadIndex` (`KismetMathLibrary.RandomIntegerInRange` 0 5))
  ;[1 1 1] SkinTexture
  (set `self.SkinTextureIndex` (`KismetMathLibrary.RandomIntegerInRange` 0 5))
  ;[1 1 1] SkinTextureModifier
  (set `self.SkinTextureModifierIndex` (`KismetMathLibrary.RandomIntegerInRange` 0 35))
  ;[1 1 1] Hair
  (set `self.HairIndex` (`KismetMathLibrary.RandomIntegerInRange` 0 4))
  ;[1 1 1] Eyebrows
  (set `self.EyebrowsIndex` (`KismetMathLibrary.RandomIntegerInRange` 0 5))
  ;[1 1 1] Mustache
  (set `self.MustacheIndex` (`KismetMathLibrary.RandomIntegerInRange` 0 3))
  ;[1 1 1] Beard
  (set `self.BeardIndex` (`KismetMathLibrary.RandomIntegerInRange` 0 2))
  ;[1 1 1] HairColor
  (set `self.HairColorIndex` (`KismetMathLibrary.RandomIntegerInRange` 0 7))
  ;[1 1 1] Outfit
  (set `self.OutfitIndex` (`KismetMathLibrary.RandomIntegerInRange` 0 14))
  ;[1 1 1] PatternOption
  (set `self.PatternOptionIndex` (`KismetMathLibrary.RandomIntegerInRange` 0 15))
  ;[1 1 1] PatternColor
  (set `self.PatternColorIndex` (`KismetMathLibrary.RandomIntegerInRange` 0 3))
  ;[1 1 1] Accessory (setting always to zero for now)
  (set `self.AccessoryIndex` 0)
  ;[1 1 1] ScaleFactor
  (set `self.ScaleFactorIndex` (`KismetMathLibrary.RandomIntegerInRange` 0 3)))

(fn `SetScalpMaterial`
  (params (MaterialInstance :type "MaterialInstanceDynamic Object Reference") (HairColorDefinition :type "/Game/CitySampleCrowd/Character/Shared/Structs/CrowdHairColorDefinition Structure") (HairDefinition :type "/Game/CitySampleCrowd/Character/Shared/Structs/CrowdHairDefinition Structure") (AttributeMapName :type Name) (FollicleMaskName :type Name) (MelaninParameterName :type Name) (RednessParameterName :type Name) (LODIndex :type Integer))
  (bind (_groom _bakedgroommap _bakedgroomminimumlod _folliclemask) (break `/Game/CitySampleCrowd/Character/Shared/Structs/CrowdHairDefinition` HairDefinition))
  (`|ExecutionSequence`
    (:`then_0`
      ;[1 1 1] Melanin and Redness
      (`self.SetMelaninAndRedless` MaterialInstance MelaninParameterName RednessParameterName HairColorDefinition))
    (:`then_1`
      ;[1 1 1] Follicle
      (`self.SetFollicleMask` MaterialInstance FollicleMaskName _folliclemask))
    (:`then_2`
      ;[1 1 1] Baked Groom Map
      (`self.SetBakedGroomMap` MaterialInstance AttributeMapName _groom _bakedgroommap _bakedgroomminimumlod LODIndex))))

(fn `SetSkeletalMesh`
  (params (SkeletalMeshComponent :type "SkeletalMeshComponent Object Reference") (SkeletalMesh :type "SkeletalMesh Soft Object Reference"))
  (bind _returnvalue (`KismetSystemLibrary.LoadAsset_Blocking` SkeletalMesh))
  (bind _asskeletal_mesh (cast `SkeletalMesh` _returnvalue)
    (:`then`
      (`SkinnedMeshComponent.SetSkinnedAssetAndUpdate` SkeletalMeshComponent _asskeletal_mesh true))
    (:`CastFailed`
      (`SkinnedMeshComponent.SetSkinnedAssetAndUpdate` SkeletalMeshComponent null true) ; Set Empty
    )))

(fn `SetSkeletalMeshes`
  (params (Base :type "SkeletalMesh Soft Object Reference") (Body :type "SkeletalMesh Soft Object Reference") (Head :type "SkeletalMesh Soft Object Reference") (Top :type "SkeletalMesh Soft Object Reference") (Bottom :type "SkeletalMesh Soft Object Reference") (Shoes :type "SkeletalMesh Soft Object Reference"))
  (`self.SetSkeletalMesh` (`self.SkeletalMesh`) Base)
  (`self.SetSkeletalMesh` (`self.Body`) Body)
  (`self.SetSkeletalMesh` (`self.Face`) Head)
  (`self.SetSkeletalMesh` (`self.Top`) Top)
  (`self.SetSkeletalMesh` (`self.Bottom`) Bottom)
  (`self.SetSkeletalMesh` (`self.Shoes`) Shoes))

(fn `SetUpdateAnimationInEditor`
  (`SkeletalMeshComponent.SetUpdateAnimationInEditor` (`self.Face`) true))

(fn `UserConstructionScript`
  ;[1 1 1] Randomize Options
  (if (`self.RandomOptions`)
    (`self.SetRandomOptions`))
  ;[1 1 1] Construct CharacterDefinition from DataAsset
  (bind _characterdefinition (`self.GetCharacterDefinition`))
  ;[1 1 1] Setting Character Definition
  (`self.SetCharacterDefinition` _characterdefinition)
  ;[1 1 1] Set Master Pose
  (`SkinnedMeshComponent.SetLeaderPoseComponent` (`self.Top`) (`self.SkeletalMesh`) false false)
  (`SkinnedMeshComponent.SetLeaderPoseComponent` (`self.Shoes`) (`self.SkeletalMesh`) false false)
  (`SkinnedMeshComponent.SetLeaderPoseComponent` (`self.Bottom`) (`self.SkeletalMesh`) false false)
  (`SkinnedMeshComponent.SetLeaderPoseComponent` (`self.Body`) (`self.SkeletalMesh`) false false)
  ;[1 1 1] Enabling Face UpdateAnimationInEditor
  (`self.SetUpdateAnimationInEditor`)
  ;[1 1 1] Disable Random
  (set `self.RandomOptions` false))